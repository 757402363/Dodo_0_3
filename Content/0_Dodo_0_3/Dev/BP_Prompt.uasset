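; BP_Prompt is an interaction prompt actor with a prepare zone and a confirm zone that react to VR hands or the PC character.
; Entering Box_Prepare unhides the BPcPrompt component and plays the prepare sound, and leaving it hides the prompt again.
; Entering Box_Confirm only plays the confirm sound.
; All three overlap events filter the other actor through casts to the left hand, right hand or PC pawn.
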(event OnComponentBeginOverlap(Box_Prepare)
  (params (OverlappedComponent :type Primitive%20Component%20Object%20Reference) (OtherActor :type Actor%20Object%20Reference) (OtherComp :type Primitive%20Component%20Object%20Reference) (OtherBodyIndex :type Integer) (bFromSweep :type Boolean) (SweepResult :type Hit%20Result%20Structure%20%28by%20ref%29))
  ;[1 1 1] 预备
  (Utilities|Casting|CastToBP_Hand_Left OtherActor
    (:then
      _)
    (:CastFailed
      (Utilities|Casting|CastToBP_Hand_Right OtherActor
        (:then
          _)
        (:CastFailed
          (Utilities|Casting|CastToBPc_PCPawn_Character OtherActor)))))
  (Development|SetHiddeninGame (Variables|Default|GetBPc_Prompt) false false)
  (Audio|Components|Audio|Play (Variables|Default|GetAudio_Prepare) 0.0))

(event OnComponentEndOverlap(Box_Prepare)
  (params (OverlappedComponent :type Primitive%20Component%20Object%20Reference) (OtherActor :type Actor%20Object%20Reference) (OtherComp :type Primitive%20Component%20Object%20Reference) (OtherBodyIndex :type Integer))
  ;[1 1 1] 预备
  (Utilities|Casting|CastToBP_Hand_Left OtherActor
    (:then
      _)
    (:CastFailed
      (Utilities|Casting|CastToBP_Hand_Right OtherActor
        (:then
          _)
        (:CastFailed
          (Utilities|Casting|CastToBPc_PCPawn_Character OtherActor)))))
  (Development|SetHiddeninGame (Variables|Default|GetBPc_Prompt) true false))

(event OnComponentBeginOverlap(Box_Confirm)
  (params (OverlappedComponent :type Primitive%20Component%20Object%20Reference) (OtherActor :type Actor%20Object%20Reference) (OtherComp :type Primitive%20Component%20Object%20Reference) (OtherBodyIndex :type Integer) (bFromSweep :type Boolean) (SweepResult :type Hit%20Result%20Structure%20%28by%20ref%29))
  ;[1 1 1] 确认
  (Utilities|Casting|CastToBP_Hand_Left OtherActor
    (:then
      _)
    (:CastFailed
      (Utilities|Casting|CastToBP_Hand_Right OtherActor
        (:then
          _)
        (:CastFailed
          (Utilities|Casting|CastToBPc_PCPawn_Character OtherActor)))))
  (Audio|Components|Audio|Play (Variables|Default|GetAudio_Confirm) 0.0))

(fn ConstructionScript)