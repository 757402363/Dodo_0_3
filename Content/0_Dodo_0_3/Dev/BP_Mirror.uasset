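; BP_Mirror is a mirror that starts invisible and switches on when a BP_Rope cable is plugged into it.
; BeginPlay creates a dynamic material instance on the mirror mesh with zero Opacity.
; When the rope's SMPortOut overlaps the hidden Cylinder trigger, the port stops simulating physics and the trigger is destroyed to prevent retriggering.
; The ShowMirror timeline then drives Opacity to reveal the mirror.
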(event OnComponentBeginOverlap(Cylinder)
  (params (OverlappedComponent :type Primitive%20Component%20Object%20Reference) (OtherActor :type Actor%20Object%20Reference) (OtherComp :type Primitive%20Component%20Object%20Reference) (OtherBodyIndex :type Integer) (bFromSweep :type Boolean) (SweepResult :type Hit%20Result%20Structure%20%28by%20ref%29))
  ;[1 1 1] 电缆的头部接口球体与隐藏圆柱体发生重叠时，取消其球体的物理模拟，销毁圆柱体避免再次触发，并开启镜子。
  (bind _asbp_rope (Utilities|Casting|CastToBP_Rope OtherActor))
  (if (== (Variables|/Game/0_Dodo_0_3/Dev/BP_Rope.BP_Rope_C|GetSM_PortOut _asbp_rope) OtherComp)
    (Physics|SetSimulatePhysics (Variables|/Game/0_Dodo_0_3/Dev/BP_Rope.BP_Rope_C|GetSM_PortOut _asbp_rope) false)
    (Components|DestroyComponent (Variables|Default|GetCylinder))
    (bind _line0 (Timeline|ShowMirror PlayFromStart)
      (:Update
        (Rendering|Material|SetScalarParameterValue (Variables|Default|GetDMI_Mirror) "Opacity" _line0 :!class /Script/Engine.MaterialInstanceDynamic)))))

(event EventBeginPlay
  ;[1 1 1] 创建动态材质实例并隐藏
  (bind _returnvalue (Rendering|Material|CreateDynamicMaterialInstance (Variables|Default|GetSM_Mirror) 0 0 "None" :!class /Script/Engine.PrimitiveComponent))
  (bind _output_get (Variables|Default|SetDMI_Mirror _returnvalue))
  (Rendering|Material|SetScalarParameterValue _output_get "Opacity" 0.0 :!class /Script/Engine.MaterialInstanceDynamic))

(fn ConstructionScript)