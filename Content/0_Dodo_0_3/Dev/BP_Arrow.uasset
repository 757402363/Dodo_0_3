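; BP_Arrow is an arrow indicator actor that scales into view and pulses its light color.
; BeginPlay creates a dynamic material instance on the SMArrow mesh.
; ShowArrow unhides the mesh and plays a timeline that drives its world scale.
; Tick flip-flops a second timeline forward and backward whenever StrengthOfLight hits either endpoint, looping a blink through the material Color's green channel.
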(event Custom|ShowArrow
  ;[1 1 1] 显示箭头指示
  (Development|SetHiddeninGame (Variables|Default|GetSM_Arrow) false false)
  (bind _line0 (Timeline|TimeLine_ShowArrow PlayFromStart)
    (:Update
      (Transformation|SetWorldScale3D (Variables|Default|GetSM_Arrow) (Math|Vector|MakeVector _line0 _line0 _line0)))))

(event EventBeginPlay
  ;[1 1 1] 创建动态材质实例
  (bind _returnvalue (Rendering|Material|CreateDynamicMaterialInstance (Variables|Default|GetSM_Arrow) 0 0 "None" :!class /Script/Engine.PrimitiveComponent))
  (Variables|Default|SetDMI_Light_Green _returnvalue))

(event EventTick
  (params (DeltaSeconds :type Float%20%28single-precision%29))
  ;[1 1 1] 指示灯光循环闪烁
  (if (or (== 5e+01 (Variables|Default|GetStrengthOfLight)) (== (Variables|Default|GetStrengthOfLight) 1e+03))
    (Utilities|FlowControl|FlipFlop
      (:A
        (bind _新建轨道_0 (Timeline|时间轴_0 PlayFromStart)
          (:Update
            (bind _output_get (Variables|Default|SetStrengthOfLight _新建轨道_0))
            (Rendering|Material|SetVectorParameterValue (Variables|Default|GetDMI_Light_Green) "Color" (Utilities|Struct|MakeLinearColor 1.0 _output_get 1.0 1.0) :!class /Script/Engine.MaterialInstanceDynamic))))
      (:B
        (Timeline|时间轴_0 ReverseFromEnd)))))

(fn ConstructionScript)