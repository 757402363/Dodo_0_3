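; BP_TestHandMaterial is a test pickup actor that assigns its hand material to PlayerController_Dodo.
; On BeginPlay, IsHandMesh selects a visible cube or sphere to display the material.
; Overlaps use only the Sphere, even when hidden, and respond to either motion controller or the PC pawn.
; They set MHandMesh, then open Map_Temp after a delay, or set MHandTracking without changing level, depending on IsHandMesh.
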(event OnComponentBeginOverlap(Sphere)
  (params (OverlappedComponent :type Primitive%20Component%20Object%20Reference) (OtherActor :type Actor%20Object%20Reference) (OtherComp :type Primitive%20Component%20Object%20Reference) (OtherBodyIndex :type Integer) (bFromSweep :type Boolean) (SweepResult :type Hit%20Result%20Structure%20%28by%20ref%29))
  ;[1 1 1] 手部与该Actor开始重叠时，根据实例设置信息设置PlayerController对应手部材质变量
  (Utilities|Casting|CastToBP_MotionController_Left OtherActor
    (:then
      _)
    (:CastFailed
      (Utilities|Casting|CastToBP_MotionController_Right OtherActor
        (:then
          _)
        (:CastFailed
          (Utilities|Casting|CastToBPc_PCPawn_Character OtherActor)))))
  (if (Variables|Default|GetIsHandMesh)
    (Variables|/Game/0_Dodo_0_3/Core/PlayerController_Dodo.PlayerController_Dodo_C|SetM_HandMesh (Variables|References|GetPlayerController_Dodo) (Variables|Default|GetHandMaterial))
    (Utilities|FlowControl|Delay 3.0)
    (Game|OpenLevel(byName) "Map_Temp")
    (else
      (Variables|/Game/0_Dodo_0_3/Core/PlayerController_Dodo.PlayerController_Dodo_C|SetM_HandTracking (Variables|References|GetPlayerController_Dodo) (Variables|Default|GetHandMaterial)))))

(event EventBeginPlay
  (Utilities|FlowControl|Sequence
    (:then_0
      ;[1 1 1] 根据实例的IsHandMesh设置显示的是球体还是立方体，再将材质设置为该几何体材质
      (if (Variables|Default|GetIsHandMesh)
        (Rendering|SetVisibility (Variables|Default|GetSphere) false false)
        (Rendering|SetVisibility (Variables|Default|GetCube) true false)
        (Rendering|Material|SetMaterial (Variables|Default|GetCube) 0 (Variables|Default|GetHandMaterial))
        (else
          (Rendering|SetVisibility (Variables|Default|GetSphere) true false)
          (Rendering|SetVisibility (Variables|Default|GetCube) false false)
          (Rendering|Material|SetMaterial (Variables|Default|GetSphere) 0 (Variables|Default|GetHandMaterial)))))
    (:then_1
      ;[1 1 1] 玩家控制器的引用
      (bind _asplayer_controller_dodo (Utilities|Casting|CastToPlayerController_Dodo (Game|GetPlayerController 0)))
      (Variables|References|SetPlayerController_Dodo _asplayer_controller_dodo))))

(fn ConstructionScript)