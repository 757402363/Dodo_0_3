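; BP_TeleportToSpaceship is a one-shot trigger that plays the transition cutscene to the large spaceship.
; When a VR or PC player pawn overlaps the box, it hides and unpossesses the pawn, then destroys the box.
; It plays the LSq_ToSpaceship sequence and calls SequenceToSpaceship on the BP_Spaceship_Large found at BeginPlay.
; Hard-coded delays time white camera fades around the cutscene; the pawn is never repossessed here.
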(event OnComponentBeginOverlap(Box)
  (params (OverlappedComponent :type Primitive%20Component%20Object%20Reference) (OtherActor :type Actor%20Object%20Reference) (OtherComp :type Primitive%20Component%20Object%20Reference) (OtherBodyIndex :type Integer) (bFromSweep :type Boolean) (SweepResult :type Hit%20Result%20Structure%20%28by%20ref%29))
  ;[0 0 0] 隐藏Pawn（避免被过场动画拍到）并解控（避免误触）
  (bind _asvrpawn_dodo (Utilities|Casting|CastToVRPawn_Dodo OtherActor)
    (:then
      (Rendering|SetActorHiddenInGame _asvrpawn_dodo true))
    (:CastFailed
      (bind _asbpc_pcpawn_character (Utilities|Casting|CastToBPc_PCPawn_Character OtherActor))
      (Rendering|SetActorHiddenInGame _asbpc_pcpawn_character true)))
  (Pawn|UnPossess (Game|GetPlayerController 0))
  (Components|DestroyComponent (Variables|Default|GetBox))
  (bind _outactor (Sequencer|Player|CreateLevelSequencePlayer "/Game/0_Dodo_0_3/Sequences/LSq_ToSpaceship.LSq_ToSpaceship"))
  (Sequencer|Player|Play (Variables|/Script/LevelSequence.LevelSequenceActor|GetSequencePlayer _outactor) :!class /Script/MovieScene.MovieSceneSequencePlayer)
  (Default|SequencetoSpaceship (Variables|References|GetSpaceship_large))
  (CameraFades|StartCameraFade (Game|GetPlayerCameraManager 0) 1.0 0.0 3.0 "(R=1.000000,G=1.000000,B=1.000000,A=1.000000)" false false)
  (Utilities|FlowControl|Delay 30.5)
  (CameraFades|StartCameraFade (Game|GetPlayerCameraManager 0) 0.0 1.0 3.0 "(R=1.000000,G=1.000000,B=1.000000,A=1.000000)" true true)
  (Utilities|FlowControl|Delay 3.0)
  (CameraFades|StartCameraFade (Game|GetPlayerCameraManager 0) 1.0 0.0 4.0 "(R=1.000000,G=1.000000,B=1.000000,A=1.000000)" true false))

(event EventBeginPlay
  ;[1 1 1] 获取飞船Actor的引用
  (bind _outactors (Actor|GetAllActorsOfClass "/Game/0_Dodo_0_3/Actors/Hologram/BP_SpaceShip_Large.BP_Spaceship_Large_C"))
  (Variables|References|SetSpaceship_large (Utilities|Array|Get(acopy) _outactors)))

(fn ConstructionScript)