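; BP_Rope is the energy cable prop that, per its guide text, plugs into a glowing wall spot to activate a self-restoring mirror.
; On BeginPlay it applies one-off forces to the port mesh and several skeletal rope bones so the cable twists naturally.
; It also spawns a BP_HoloGuide_Box with Chinese name and description text, snap-attached to an arrow component.
; The plug-in and mirror logic are not in this graph.
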(event EventBeginPlay
  ;[1 1 1] 给绳子添加一个初始的作用力，使其扭曲更像一条绳子
  (Utilities|FlowControl|Sequence
    (:then_0
      (Physics|AddForce (Variables|Default|GetSM_PortOut) "-5000.000000,-5000.000000,-40000.000000" "None" false)
      (Physics|AddForce (Variables|Default|GetSkM_Rope) "-3000.000000,-3000.000000, 0" "Bone_200" false)
      (Physics|AddForce (Variables|Default|GetSkM_Rope) "-3000.000000, 0, 0" "Bone_250" false)
      (Physics|AddForce (Variables|Default|GetSkM_Rope) "0.000000,-3000.000000, 0" "Bone_300" false))
    (:then_1
      ;[1 1 1] 设置引导Box文本内容，并对齐箭头变换附加到箭头
      (bind _returnvalue (Game|SpawnActorfromClass "/Game/0_Dodo_0_3/Actors/HoloGuide/BP_HoloGuide_Box.BP_HoloGuide_Box_C" (Transformation|GetWorldTransform (Variables|Default|GetArrow_HoloGuide_Box)) "AlwaysSpawn" 0 0))
      (Variables|/Game/0_Dodo_0_3/Actors/HoloGuide/BP_HoloGuide_Box.BP_HoloGuide_Box_C|SetText_Name _returnvalue "能量缆线")
      (Variables|/Game/0_Dodo_0_3/Actors/HoloGuide/BP_HoloGuide_Box.BP_HoloGuide_Box_C|SetText_Description _returnvalue "将头部的能量球接入墙壁发光处，以激活一面特殊的镜子，该镜子在破碎后可自动复原。")
      (Transformation|AttachComponentToComponent _returnvalue (Variables|Default|GetArrow_HoloGuide_Box) "None" "SnapToTarget" "SnapToTarget" "SnapToTarget" true))))

(fn ConstructionScript)