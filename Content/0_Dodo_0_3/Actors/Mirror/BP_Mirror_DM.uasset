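; BP_Mirror_DM is a breakable mirror actor that respawns itself after it shatters.
; At BeginPlay it takes the first SceneCapture2D found in the level and hides its own components from that capture.
; When its destructible mesh fractures, it waits ten seconds, spawns a fresh copy at the same transform, then destroys itself.
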(event OnComponentFracture(SM_Mirror_DM)
  (params (HitPoint :type Vector%20%28by%20ref%29 :default "0, 0, 0") (HitDirection :type Vector%20%28by%20ref%29 :default "0, 0, 0"))
  ;[1 1 1] 破碎后，延迟10s，在原位置生成新的该Actor，并销毁原Actor
  (Utilities|FlowControl|Delay 1e+01)
  (Game|SpawnActorfromClass "BP_Mirror_DM_C" (Transformation|GetActorTransform) "AlwaysSpawn" 0 0)
  (Actor|DestroyActor))

(event EventBeginPlay
  ;[1 1 1] 获取对场景捕获2D的引用，并设置其对本Actor的隐藏
  (bind _outactors (Actor|GetAllActorsOfClass "/Script/Engine.SceneCapture2D"))
  (bind _output_get (Variables|Default|SetRef_SceneCapture2D (Utilities|Array|Get(acopy) _outactors)))
  (Class|SceneCaptureComponent|HideActorComponents (Variables|/Script/Engine.SceneCapture2D|GetCaptureComponent2D _output_get) self false))

(fn ConstructionScript)