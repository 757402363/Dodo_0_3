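; BP_Mirror_Spawn is a trigger actor that spawns a breakable mirror once a rope cable's head connector reaches it.
; When BP_Rope's SMPortOut overlaps the Cylinder, the connector stops simulating physics and the Cylinder is destroyed to prevent retriggering.
; BP_Mirror_DM spawns at the arrow transform, briefly hidden until its dynamic material is transparent, then the ShowMirror timeline drives Opacity to reveal it.
; BeginPlay holds only an unconnected test delay.
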(event OnComponentBeginOverlap(Cylinder)
  (params (OverlappedComponent :type Primitive%20Component%20Object%20Reference) (OtherActor :type Actor%20Object%20Reference) (OtherComp :type Primitive%20Component%20Object%20Reference) (OtherBodyIndex :type Integer) (bFromSweep :type Boolean) (SweepResult :type Hit%20Result%20Structure%20%28by%20ref%29))
  ;[1 1 1] 电缆的头部接口球体与隐藏圆柱体发生重叠时，取消其球体的物理模拟，销毁隐藏圆柱体避免再次触发。
  (bind _asbp_rope (Utilities|Casting|CastToBP_Rope OtherActor))
  (if (== (Variables|/Game/0_Dodo_0_3/Actors/Mirror/BP_Rope.BP_Rope_C|GetSM_PortOut _asbp_rope) OtherComp)
    (Physics|SetSimulatePhysics (Variables|/Game/0_Dodo_0_3/Actors/Mirror/BP_Rope.BP_Rope_C|GetSM_PortOut _asbp_rope) false)
    (Components|DestroyComponent (Variables|Default|GetCylinder))
    ;[1 1 1] 生成会破碎的镜子，并使其逐渐显形
    (bind _returnvalue (Game|SpawnActorfromClass "/Game/0_Dodo_0_3/Actors/Mirror/BP_Mirror_DM.BP_Mirror_DM_C" (Transformation|GetWorldTransform (Variables|Default|GetArrow_SpawnMirror)) "AlwaysSpawn" 0 0))
    (Rendering|SetActorHiddenInGame _returnvalue true)
    (Utilities|FlowControl|Delay 0.1)
    (bind _returnvalue_2 (Rendering|Material|CreateDynamicMaterialInstance (Variables|/Game/0_Dodo_0_3/Actors/Mirror/BP_Mirror_DM.BP_Mirror_DM_C|GetSM_Mirror_DM _returnvalue) 1 0 "None" :!class /Script/Engine.PrimitiveComponent))
    (bind _output_get (Variables|Default|SetDMI_Mirror _returnvalue_2))
    (Rendering|Material|SetScalarParameterValue _output_get "Opacity" 0.0 :!class /Script/Engine.MaterialInstanceDynamic)
    (Rendering|SetActorHiddenInGame _returnvalue false)
    (bind _line0 (Timeline|ShowMirror PlayFromStart)
      (:Update
        (Rendering|Material|SetScalarParameterValue (Variables|Default|GetDMI_Mirror) "Opacity" _line0 :!class /Script/Engine.MaterialInstanceDynamic)))))

(event EventBeginPlay
  ;[1 1 0] PCPawn测试，延迟后生成镜子（考虑前置条件需要时间）
  (Utilities|FlowControl|Delay 5.0))

(fn ConstructionScript)