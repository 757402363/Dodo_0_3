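; BP_SpawnProps is a button actor that spawns a configurable prop when a VR hand or player character overlaps its Cube.
; Props spawn just above it with randomized rotation around an arrow's yaw and random per-axis scale.
; Slime, cup and mannequin props get a randomized, mostly upward force, followed by a short cooldown.
; An optional looping timer on BeginPlay provides auto-spawning for testing.
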(event OnComponentBeginOverlap(Cube)
  (params (OverlappedComponent :type Primitive%20Component%20Object%20Reference) (OtherActor :type Actor%20Object%20Reference) (OtherComp :type Primitive%20Component%20Object%20Reference) (OtherBodyIndex :type Integer) (bFromSweep :type Boolean) (SweepResult :type Hit%20Result%20Structure%20%28by%20ref%29))
  (bind _returnvalue (Math|Random|RandomFloatinRange -3e+01 3e+01))
  (bind _scale_min (Variables|Default|GetScale_Min))
  (bind _scale_max (Variables|Default|GetScale_Max))
  (bind _forcez (Variables|Default|GetForceZ))
  (bind _arrow_rotationz (Variables|Default|GetArrow_RotationZ))
  (bind _returnvalue_2 (/ _forcez 6.0))
  (bind _returnvalue_3 (Transformation|GetWorldRotation _arrow_rotationz))
  (bind _returnvalue_4 (Math|Random|RandomFloatinRange _scale_min _scale_max))
  (bind _returnvalue_5 (Math|Random|RandomFloatinRange 0.0 _returnvalue_2))
  ;[1 1 1] 按下按钮，生成所需道具并添加大致向上的作用力，道具的旋转、缩放以及施加作用力的大小和方向都在一定范围内随机
  (if (Variables|Default|GetSpawnAllow)
    (Utilities|Casting|CastToBP_Hand_Left OtherActor
      (:then
        _)
      (:CastFailed
        (Utilities|Casting|CastToBP_Hand_Right OtherActor
          (:then
            _)
          (:CastFailed
            (Utilities|Casting|CastToBPc_PCPawn_Character OtherActor)))))
    (bind _returnvalue_6 (Game|SpawnActorfromClass (Variables|Default|GetProp) (Math|Transform|MakeTransform (+ (Transformation|GetActorLocation) "0, 0,25.000000") (Math|Rotator|MakeRotator _returnvalue _returnvalue (Math|Random|RandomFloatinRange (- (.yaw _returnvalue_3) 3e+01) (+ (.yaw _returnvalue_3) 3e+01))) (Math|Vector|MakeVector _returnvalue_4 _returnvalue_4 _returnvalue_4)) "AdjustIfPossibleButAlwaysSpawn" 0 0))
    (bind _asbp_slime (Utilities|Casting|CastToBP_Slime _returnvalue_6)
      (:then
        (Physics|AddForce (Variables|/Game/0_Dodo_0_3/Actors/SpawnProps/BP_Slime.BP_Slime_C|GetSkM_Slime _asbp_slime) (Math|Vector|MakeVector _returnvalue_5 _returnvalue_5 _forcez) "None" false))
      (:CastFailed
        (bind _asbp_cup (Utilities|Casting|CastToBP_Cup _returnvalue_6)
          (:then
            (Physics|AddForce (Variables|/Game/0_Dodo_0_3/Actors/SpawnProps/BP_Cup.BP_Cup_C|GetSM_GlassCup _asbp_cup) (Math|Vector|MakeVector _returnvalue_5 _returnvalue_5 _forcez) "None" false))
          (:CastFailed
            (bind _asbp_mannequin (Utilities|Casting|CastToBP_Mannequin _returnvalue_6))
            (Physics|AddForce (Variables|/Game/0_Dodo_0_3/Actors/SpawnProps/BP_Mannequin.BP_Mannequin_C|GetSkM_Mannequin _asbp_mannequin) (Math|Vector|MakeVector _returnvalue_5 _returnvalue_5 _forcez) "None" false)))))
    (Variables|Default|SetSpawnAllow false)
    (Utilities|FlowControl|Delay 1.0)
    (Variables|Default|SetSpawnAllow true)))

(event Custom|Test_SpawnProps_Auto
  (bind _returnvalue (Math|Random|RandomFloatinRange -3e+01 3e+01))
  (bind _scale_min (Variables|Default|GetScale_Min))
  (bind _scale_max (Variables|Default|GetScale_Max))
  (bind _forcez (Variables|Default|GetForceZ))
  (bind _arrow_rotationz (Variables|Default|GetArrow_RotationZ))
  (bind _returnvalue_2 (/ _forcez 6.0))
  (bind _returnvalue_3 (Transformation|GetWorldRotation _arrow_rotationz))
  (bind _returnvalue_4 (Math|Random|RandomFloatinRange _scale_min _scale_max))
  (bind _returnvalue_5 (Math|Random|RandomFloatinRange 0.0 _returnvalue_2))
  ;[1 1 0] 测试，用于自动生成道具
  ;[1 1 1] 按下按钮，生成所需道具并添加大致向上的作用力，道具的旋转、缩放以及施加作用力的大小和方向都在一定范围内随机
  (bind _returnvalue_6 (Game|SpawnActorfromClass (Variables|Default|GetProp) (Math|Transform|MakeTransform (+ (Transformation|GetActorLocation) "0, 0,25.000000") (Math|Rotator|MakeRotator _returnvalue _returnvalue (Math|Random|RandomFloatinRange (- (.yaw _returnvalue_3) 3e+01) (+ (.yaw _returnvalue_3) 3e+01))) (Math|Vector|MakeVector _returnvalue_4 _returnvalue_4 _returnvalue_4)) "AdjustIfPossibleButAlwaysSpawn" 0 0))
  (bind _asbp_slime (Utilities|Casting|CastToBP_Slime _returnvalue_6)
    (:then
      (Physics|AddForce (Variables|/Game/0_Dodo_0_3/Actors/SpawnProps/BP_Slime.BP_Slime_C|GetSkM_Slime _asbp_slime) (Math|Vector|MakeVector _returnvalue_5 _returnvalue_5 _forcez) "None" false))
    (:CastFailed
      (bind _asbp_cup (Utilities|Casting|CastToBP_Cup _returnvalue_6)
        (:then
          (Physics|AddForce (Variables|/Game/0_Dodo_0_3/Actors/SpawnProps/BP_Cup.BP_Cup_C|GetSM_GlassCup _asbp_cup) (Math|Vector|MakeVector _returnvalue_5 _returnvalue_5 _forcez) "None" false))
        (:CastFailed
          (bind _asbp_mannequin (Utilities|Casting|CastToBP_Mannequin _returnvalue_6))
          (Physics|AddForce (Variables|/Game/0_Dodo_0_3/Actors/SpawnProps/BP_Mannequin.BP_Mannequin_C|GetSkM_Mannequin _asbp_mannequin) (Math|Vector|MakeVector _returnvalue_5 _returnvalue_5 _forcez) "None" false)))))
  (Variables|Default|SetSpawnAllow false)
  (Utilities|FlowControl|Delay 1.0)
  (Variables|Default|SetSpawnAllow true))

(event EventBeginPlay
  ;[1 1 1] 设置按钮材质
  (Rendering|Material|SetMaterial (Variables|Default|GetSM_Button) 0 (Variables|Default|GetColorOfButton))
  ;[1 1 0] 测试，用于自动生成道具
  (if (Variables|Default|GetAutoSpawn)
    (Utilities|Time|SetTimerbyEvent (EventDispatchers|CreateEvent :!event Custom|Test_SpawnProps_Auto) 2.0 true)))

(fn ConstructionScript)