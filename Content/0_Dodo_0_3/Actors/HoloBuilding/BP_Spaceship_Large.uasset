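; BP_Spaceship_Large is a large spaceship actor, filed with the holo building assets, that plays its part in a cutscene.
; The Sequence_ToSpaceship event starts the ship's audio cue after a short delay.
; After a longer delay it hides the teleport effect component with its children and reveals the engine flame effects for main power and left and right yaw.
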(event Custom|Sequence_ToSpaceship
  ;[1 1 1] 过场动画变化内容
  ;;[0 0 0] 飞船音效
  (Utilities|FlowControl|Delay 5.0)
  (Audio|Components|Audio|Play (Variables|Default|GetCue_Spaceship) 0.0)
  ;;[0 0 0] 隐藏传送特效，显示尾焰特效
  (Utilities|FlowControl|Delay 28.5)
  (Development|SetHiddeninGame (Variables|Default|GetActorComp_Teleport) true true)
  (Development|SetHiddeninGame (Variables|Default|GetP_Power1) false false))

(fn ConstructionScript)