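; BP_SetHandMaterial is a touchable swatch actor that changes the player's hand material.
; IsHandMesh picks a visible cube (hand mesh) or sphere (hand tracking) to preview HandMaterial.
; Sphere overlap by either hand or the PC pawn plays a scale-up timeline, then audio and a scale-down.
; Between timelines, it writes the material to the matching GameInstance_Dodo variable and broadcasts ChangeHandMaterial.
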(event OnComponentBeginOverlap(Sphere)
  (params (OverlappedComponent :type Primitive%20Component%20Object%20Reference) (OtherActor :type Actor%20Object%20Reference) (OtherComp :type Primitive%20Component%20Object%20Reference) (OtherBodyIndex :type Integer) (bFromSweep :type Boolean) (SweepResult :type Hit%20Result%20Structure%20%28by%20ref%29))
  ;[1 1 1] 手部与该材质几何体开始重叠时，根据实例设置信息设置GameInstance对应手部材质接口变量，并调用事件分发器进行通知（几何体放大变小并伴随声音，形成反馈）
  (Utilities|Casting|CastToBP_Hand_Left OtherActor
    (:then
      (bind _line0 (Timeline|Scale1 PlayFromStart)
        (:Update
          (Transformation|SetWorldScale3D (Variables|Default|GetSphere) (Math|Vector|MakeVector _line0 _line0 _line0)))
        (:Finished
          (Audio|Components|Audio|Play (Variables|Default|GetAudio) 0.0)
          (if (Variables|Default|GetIsHandMesh)
            (Variables|/Game/0_Dodo_0_3/Core/GameInstance_Dodo.GameInstance_Dodo_C|SetM_HandMesh (Variables|References|GetGameInstance_Dodo) (Variables|Default|GetHandMaterial))
            (else
              (Variables|/Game/0_Dodo_0_3/Core/GameInstance_Dodo.GameInstance_Dodo_C|SetM_HandTracking (Variables|References|GetGameInstance_Dodo) (Variables|Default|GetHandMaterial))))
          (Default|CallChangeHandMaterial (Variables|References|GetGameInstance_Dodo))
          (bind _line0_2 (Timeline|Scale2 PlayFromStart)
            (:Update
              (Transformation|SetWorldScale3D (Variables|Default|GetSphere) (Math|Vector|MakeVector _line0_2 _line0_2 _line0_2)))))))
    (:CastFailed
      (Utilities|Casting|CastToBP_Hand_Right OtherActor
        (:then
          (Timeline|Scale1 PlayFromStart))
        (:CastFailed
          (Utilities|Casting|CastToBPc_PCPawn_Character OtherActor)
          (Timeline|Scale1 PlayFromStart))))))

(event EventBeginPlay
  (Utilities|FlowControl|Sequence
    (:then_0
      ;[1 1 1] 根据实例的IsHandMesh设置显示的是球体还是立方体，再将材质设置为该几何体材质
      (if (Variables|Default|GetIsHandMesh)
        (Rendering|SetVisibility (Variables|Default|GetSphere) false false)
        (Rendering|SetVisibility (Variables|Default|GetCube) true false)
        (Rendering|Material|SetMaterial (Variables|Default|GetCube) 0 (Variables|Default|GetHandMaterial))
        (else
          (Rendering|SetVisibility (Variables|Default|GetSphere) true false)
          (Rendering|SetVisibility (Variables|Default|GetCube) false false)
          (Rendering|Material|SetMaterial (Variables|Default|GetSphere) 0 (Variables|Default|GetHandMaterial)))))
    (:then_1
      ;[1 1 1] 游戏实例的引用
      (bind _asgame_instance_dodo (Utilities|Casting|CastToGameInstance_Dodo (Game|GetGameInstance)))
      (Variables|References|SetGameInstance_Dodo _asgame_instance_dodo))))

(fn ConstructionScript)