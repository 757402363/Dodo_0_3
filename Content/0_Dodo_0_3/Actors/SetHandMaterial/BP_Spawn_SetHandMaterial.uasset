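; BP_Spawn_SetHandMaterial is a touch button that shows or hides a set of hand-material option actors (three Tracking, three Mesh).
; On BeginPlay it hides these child actors and teleports them upward out of reach to prevent accidental touches.
; When the left hand, right hand or PC pawn overlaps the Cube, a FlipFlop alternately brings them down visible or lifts them away hidden, with no actual spawning.
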(event OnComponentBeginOverlap(Cube)
  (params (OverlappedComponent :type Primitive%20Component%20Object%20Reference) (OtherActor :type Actor%20Object%20Reference) (OtherComp :type Primitive%20Component%20Object%20Reference) (OtherBodyIndex :type Integer) (bFromSweep :type Boolean) (SweepResult :type Hit%20Result%20Structure%20%28by%20ref%29))
  (bind _tracking1 (Variables|Default|GetTracking1))
  (bind _tracking3 (Variables|Default|GetTracking3))
  ;[1 1 1] 触碰按钮，状态切换
  (Utilities|Casting|CastToBP_Hand_Left OtherActor
    (:then
      _)
    (:CastFailed
      (Utilities|Casting|CastToBP_Hand_Right OtherActor
        (:then
          _)
        (:CastFailed
          (Utilities|Casting|CastToBPc_PCPawn_Character OtherActor)))))
  (Utilities|FlowControl|FlipFlop
    (:A
      (Transformation|AddWorldOffset _tracking3 "0, 0,-1000.000000" false true)
      (Development|SetHiddeninGame _tracking3 false false))
    (:B
      (Transformation|AddWorldOffset _tracking1 "0, 0,1000.000000" false true)
      (Development|SetHiddeninGame _tracking1 true false))))

(event EventBeginPlay
  ;[1 1 1] 隐藏并偏移子Actor，避免误触
  (Transformation|AddWorldOffset (Variables|Default|GetTracking2) "0, 0,1000.000000" false true)
  (Development|SetHiddeninGame (Variables|Default|GetTracking1) true false))

(fn ConstructionScript)