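; BP_HoloGuide_Box is a trigger box actor that shows an animated prompt indicator when the HoloGuide reaches it.
; Box overlap events unhide Prompt when BP_HoloGuide's CapsuleTrace component enters and hide it again when that component leaves, ignoring its other components.
; A looping timer set on BeginPlay and the PromptScale timeline event give the prompt a repeating uniform scale animation.
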(event OnComponentBeginOverlap(Box)
  (params (OverlappedComponent :type Primitive%20Component%20Object%20Reference) (OtherActor :type Actor%20Object%20Reference) (OtherComp :type Primitive%20Component%20Object%20Reference) (OtherBodyIndex :type Integer) (bFromSweep :type Boolean) (SweepResult :type Hit%20Result%20Structure%20%28by%20ref%29))
  ;[1 1 1] 如果Box与检测胶囊体重叠，显示指示框，反之隐藏。
  (bind _asbp_holo_guide (Utilities|Casting|CastToBP_HoloGuide OtherActor))
  (if (== (Variables|/Game/0_Dodo_0_3/Actors/HoloGuide/BP_HoloGuide.BP_HoloGuide_C|GetCapsule_Trace _asbp_holo_guide) OtherComp)
    (Development|SetHiddeninGame (Variables|Default|GetPrompt) false false)))

(event OnComponentEndOverlap(Box)
  (params (OverlappedComponent :type Primitive%20Component%20Object%20Reference) (OtherActor :type Actor%20Object%20Reference) (OtherComp :type Primitive%20Component%20Object%20Reference) (OtherBodyIndex :type Integer))
  ;[1 1 1] 如果Box与检测胶囊体重叠，显示指示框，反之隐藏。
  (bind _asbp_holo_guide (Utilities|Casting|CastToBP_HoloGuide OtherActor))
  (if (== (Variables|/Game/0_Dodo_0_3/Actors/HoloGuide/BP_HoloGuide.BP_HoloGuide_C|GetCapsule_Trace _asbp_holo_guide) OtherComp)
    (Development|SetHiddeninGame (Variables|Default|GetPrompt) true false)))

(event Custom|PromptScale
  ;[1 1 1] 指示框循环缩放
  (bind _line0 (Timeline|PromptScaleLoop PlayFromStart)
    (:Update
      (Transformation|SetRelativeScale3D (Variables|Default|GetPrompt) (Math|Vector|MakeVector _line0 _line0 _line0)))))

(event EventBeginPlay
  ;[1 1 1] 指示框循环缩放
  (Utilities|Time|SetTimerbyEvent (EventDispatchers|CreateEvent :!event Custom|PromptScale) 2.0 true))

(fn ConstructionScript)