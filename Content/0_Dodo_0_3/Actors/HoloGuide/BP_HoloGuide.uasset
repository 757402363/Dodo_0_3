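; VR holographic guide helmet that the player wears to read names and descriptions of guide boxes.
; A rotating arrow prompt disappears when a hand nears; HoloGuide_Wear then attaches the owner-hidden helmet to the pawn and fades in a per-eye UMG intro, offset for Oculus.
; Afterwards, a capsule overlapping BP_HoloGuide_Box actors fills the text.
; Hand touches on the toggle box fade the overlay and helmet material via timelines.
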(event OnComponentBeginOverlap(Box_Prompt)
  (params (OverlappedComponent :type Primitive%20Component%20Object%20Reference) (OtherActor :type Actor%20Object%20Reference) (OtherComp :type Primitive%20Component%20Object%20Reference) (OtherBodyIndex :type Integer) (bFromSweep :type Boolean) (SweepResult :type Hit%20Result%20Structure%20%28by%20ref%29))
  ;[1 1 1] 手靠近头盔，提示相关组件销毁
  (Utilities|Casting|CastToBP_Hand_Left OtherActor
    (:then
      _)
    (:CastFailed
      (Utilities|Casting|CastToBP_Hand_Right OtherActor)))
  (Utilities|Time|ClearandInvalidateTimerbyHandle (Variables|Timers|GetTimer_ArrowRotating))
  (Components|DestroyComponent (Variables|Default|GetBox_Prompt)))

(event OnComponentBeginOverlap(Capsule_Trace)
  (params (OverlappedComponent :type Primitive%20Component%20Object%20Reference) (OtherActor :type Actor%20Object%20Reference) (OtherComp :type Primitive%20Component%20Object%20Reference) (OtherBodyIndex :type Integer) (bFromSweep :type Boolean) (SweepResult :type Hit%20Result%20Structure%20%28by%20ref%29))
  ;[1 1 1] 检测到Box将其文本变量导入UMG对应组件，结束重叠时将文本组件的内容清空。
  (if (Variables|State|GetGuideAllow)
    (bind _asbp_holo_guide_box (Utilities|Casting|CastToBP_HoloGuide_Box OtherActor))
    (Rendering|Components|TextRender|SetText (Variables|/Game/0_Dodo_0_3/UI/UMG/UMG_HoloGuide_SingleEye.UMG_HoloGuide_SingleEye_C|GetText_Name (Variables|/Game/0_Dodo_0_3/UI/UMG/UMG_HoloGuide_VDLink.UMG_HoloGuide_VDLink_C|GetUMG_HoloGuide_LeftEye (Variables|References|GetUMG_HoloGuide))) (Variables|/Game/0_Dodo_0_3/Actors/HoloGuide/BP_HoloGuide_Box.BP_HoloGuide_Box_C|GetText_Name _asbp_holo_guide_box))
    (Rendering|Components|TextRender|SetText (Variables|/Game/0_Dodo_0_3/UI/UMG/UMG_HoloGuide_SingleEye.UMG_HoloGuide_SingleEye_C|GetText_Description (Variables|/Game/0_Dodo_0_3/UI/UMG/UMG_HoloGuide_VDLink.UMG_HoloGuide_VDLink_C|GetUMG_HoloGuide_LeftEye (Variables|References|GetUMG_HoloGuide))) (Variables|/Game/0_Dodo_0_3/Actors/HoloGuide/BP_HoloGuide_Box.BP_HoloGuide_Box_C|GetText_Description _asbp_holo_guide_box))
    (Widget|SetRenderOpacity (Variables|/Game/0_Dodo_0_3/UI/UMG/UMG_HoloGuide_SingleEye.UMG_HoloGuide_SingleEye_C|GetImage_Guide_Back1 (Variables|/Game/0_Dodo_0_3/UI/UMG/UMG_HoloGuide_VDLink.UMG_HoloGuide_VDLink_C|GetUMG_HoloGuide_LeftEye (Variables|References|GetUMG_HoloGuide))) 1.0)))

(event OnComponentEndOverlap(Capsule_Trace)
  (params (OverlappedComponent :type Primitive%20Component%20Object%20Reference) (OtherActor :type Actor%20Object%20Reference) (OtherComp :type Primitive%20Component%20Object%20Reference) (OtherBodyIndex :type Integer))
  ;[1 1 1] 检测到Box将其文本变量导入UMG对应组件，结束重叠时将文本组件的内容清空。
  (if (Variables|State|GetGuideAllow)
    (Utilities|Casting|CastToBP_HoloGuide_Box OtherActor)
    (Rendering|Components|TextRender|SetText (Variables|/Game/0_Dodo_0_3/UI/UMG/UMG_HoloGuide_SingleEye.UMG_HoloGuide_SingleEye_C|GetText_Name (Variables|/Game/0_Dodo_0_3/UI/UMG/UMG_HoloGuide_VDLink.UMG_HoloGuide_VDLink_C|GetUMG_HoloGuide_LeftEye (Variables|References|GetUMG_HoloGuide))) "")
    (Widget|SetRenderOpacity (Variables|/Game/0_Dodo_0_3/UI/UMG/UMG_HoloGuide_SingleEye.UMG_HoloGuide_SingleEye_C|GetImage_Guide_Back1 (Variables|/Game/0_Dodo_0_3/UI/UMG/UMG_HoloGuide_VDLink.UMG_HoloGuide_VDLink_C|GetUMG_HoloGuide_LeftEye (Variables|References|GetUMG_HoloGuide))) 0.0)))

(event OnComponentBeginOverlap(Box_ToggleState)
  (params (OverlappedComponent :type Primitive%20Component%20Object%20Reference) (OtherActor :type Actor%20Object%20Reference) (OtherComp :type Primitive%20Component%20Object%20Reference) (OtherBodyIndex :type Integer) (bFromSweep :type Boolean) (SweepResult :type Hit%20Result%20Structure%20%28by%20ref%29))
  ;[1 1 1] 触碰头盔两侧以切换引导状态（激活或关闭）
  ;;[0 0 0] 前置判断条件
  (if (Variables|State|GetGuideAllow)
    (if (Variables|State|GetToggleStateAllow)
      (Utilities|Casting|CastToBP_Hand_Left OtherActor
        (:then
          _)
        (:CastFailed
          (Utilities|Casting|CastToBP_Hand_Right OtherActor)))
      ;;[0 0 0] 避免再次触发状态切换
      (Variables|State|SetToggleStateAllow false)
      (Utilities|FlowControl|FlipFlop
        (:A
          ;;[0 0 0] 隐藏引导文本，UMG和头盔材质逐渐透明
          (Widget|SetVisibility (Variables|/Game/0_Dodo_0_3/UI/UMG/UMG_HoloGuide_SingleEye.UMG_HoloGuide_SingleEye_C|GetText_Name (Variables|/Game/0_Dodo_0_3/UI/UMG/UMG_HoloGuide_VDLink.UMG_HoloGuide_VDLink_C|GetUMG_HoloGuide_LeftEye (Variables|References|GetUMG_HoloGuide))) "Hidden")
          (bind _line0 (Timeline|HideVfx PlayFromStart)
            (:Update
              (Widget|SetRenderOpacity (Variables|/Game/0_Dodo_0_3/UI/UMG/UMG_HoloGuide_VDLink.UMG_HoloGuide_VDLink_C|GetImage_BaseColor (Variables|References|GetUMG_HoloGuide)) _line0)
              (Rendering|Material|SetScalarParameterValue (Variables|DMI|GetDMI_HoloGuide1) "Opacity" (* _line0 0.1) :!class /Script/Engine.MaterialInstanceDynamic))
            (:Finished
              ;;[0 0 0] 允许再次触发状态切换
              (Variables|State|SetToggleStateAllow true :!label _label))))
        (:B
          ;;[0 0 0] UMG和头盔材质逐渐显现，引导文本可视
          (bind _line0_2 (Timeline|ShowVfx PlayFromStart)
            (:Update
              (Widget|SetRenderOpacity (Variables|/Game/0_Dodo_0_3/UI/UMG/UMG_HoloGuide_VDLink.UMG_HoloGuide_VDLink_C|GetImage_BaseColor (Variables|References|GetUMG_HoloGuide)) _line0_2)
              (Rendering|Material|SetScalarParameterValue (Variables|DMI|GetDMI_HoloGuide1) "Opacity" (* _line0_2 0.1) :!class /Script/Engine.MaterialInstanceDynamic))
            (:Finished
              (Widget|SetVisibility (Variables|/Game/0_Dodo_0_3/UI/UMG/UMG_HoloGuide_SingleEye.UMG_HoloGuide_SingleEye_C|GetText_Name (Variables|/Game/0_Dodo_0_3/UI/UMG/UMG_HoloGuide_VDLink.UMG_HoloGuide_VDLink_C|GetUMG_HoloGuide_LeftEye (Variables|References|GetUMG_HoloGuide))) "Visible")
              (goto _label))))))))

(event Custom|ArrowRotating
  ;[1 1 1] 箭头旋转
  (Transformation|AddLocalRotation (Variables|Default|GetSM_Arrow_Prompt) "2.000000, 0, 0" false false))

(event Custom|HoloGuide_Wear
  (bind _sm_hologuide (Variables|Default|GetSM_HoloGuide))
  ;[1 1 1] 佩戴头盔以及首次引导
  ;;[0 0 0] 取消模拟物理与碰撞，将头盔附加到VRPawn的对应箭头处
  (Physics|SetSimulatePhysics _sm_hologuide false)
  (Collision|SetCollisionEnabled _sm_hologuide "NoCollision")
  (Transformation|AttachComponentToComponent (Variables|/Game/0_Dodo_0_3/Characters/VRPawn/VRPawn_Dodo.VRPawn_Dodo_C|GetArrow_HoloGuide (Variables|References|GetVRPawn_Dodo)) "None" "SnapToTarget" "SnapToTarget" "SnapToTarget" true)
  ;;[0 0 0] 设置VRPawn为该Actor的拥有者，使头盔能对VRPawn设置拥有者不可见。
  (Actor|SetOwner (Variables|References|GetVRPawn_Dodo))
  (Class|PrimitiveComponent|SetOwnerNoSee (Variables|Default|GetSM_HoloGuide) true)
  ;;[0 0 0] UMG控件设置初始状态（底色、全息特效、初次引导文本渲染不透明度为0，引导文本清空），并添加到视口
  (bind _returnvalue (UserInterface|CreateWidget "/Game/0_Dodo_0_3/UI/UMG/UMG_HoloGuide_VDLink.UMG_HoloGuide_VDLink_C"))
  (Variables|References|SetUMG_HoloGuide _returnvalue)
  (Widget|SetRenderOpacity (Variables|/Game/0_Dodo_0_3/UI/UMG/UMG_HoloGuide_VDLink.UMG_HoloGuide_VDLink_C|GetImage_BaseColor (Variables|References|GetUMG_HoloGuide)) 0.0)
  (Rendering|Components|TextRender|SetText (Variables|/Game/0_Dodo_0_3/UI/UMG/UMG_HoloGuide_SingleEye.UMG_HoloGuide_SingleEye_C|GetText_Name (Variables|/Game/0_Dodo_0_3/UI/UMG/UMG_HoloGuide_VDLink.UMG_HoloGuide_VDLink_C|GetUMG_HoloGuide_LeftEye (Variables|References|GetUMG_HoloGuide))) "")
  (UserInterface|Viewport|AddtoViewport (Variables|References|GetUMG_HoloGuide) 0)
  ;;[0 0 0] 如果推测为Oculus官方串流，则左眼视野右移100，否则不变。
  (switch name (Class|HeadMountedDisplayFunctionLibrary|GetHMDDeviceName)
    (:Default
      ;;[0 0 0] 逐渐显示全息特效，停顿2s再逐渐显示首次佩戴引导，逐渐隐藏首次引导，然后设置允许正常引导。
      (bind _line0 (Timeline|ShowFirstVfx PlayFromStart)
        (:Update
          (Widget|SetRenderOpacity (Variables|/Game/0_Dodo_0_3/UI/UMG/UMG_HoloGuide_VDLink.UMG_HoloGuide_VDLink_C|GetImage_BaseColor (Variables|References|GetUMG_HoloGuide)) _line0))
        (:Finished
          (Utilities|FlowControl|Delay 2.0)
          (bind _line0_2 (Timeline|ShowFirstGuide PlayFromStart)
            (:Update
              (Widget|SetRenderOpacity (Variables|/Game/0_Dodo_0_3/UI/UMG/UMG_HoloGuide_SingleEye.UMG_HoloGuide_SingleEye_C|GetText_FirstGuide1 (Variables|/Game/0_Dodo_0_3/UI/UMG/UMG_HoloGuide_VDLink.UMG_HoloGuide_VDLink_C|GetUMG_HoloGuide_LeftEye (Variables|References|GetUMG_HoloGuide))) _line0_2))
            (:Finished
              (Variables|State|SetGuideAllow true))))))
    (:OculusHMD
      (Class|Widget|SetRenderTranslation (Variables|/Game/0_Dodo_0_3/UI/UMG/UMG_HoloGuide_VDLink.UMG_HoloGuide_VDLink_C|GetUMG_HoloGuide_LeftEye (Variables|References|GetUMG_HoloGuide)) "(X=100.000000,Y=0.000000)")
      (Timeline|ShowFirstVfx PlayFromStart))
    (:SteamVR
      (Timeline|ShowFirstVfx PlayFromStart))))

(event EventBeginPlay
  (Utilities|FlowControl|Sequence
    (:then_0
      ;[1 1 1] 获取VRPawn引用
      (Utilities|FlowControl|Delay 0.1)
      (bind _asvrpawn_dodo (Utilities|Casting|CastToVRPawn_Dodo (Game|Player|GetPlayerPawn 0)))
      (Variables|References|SetVRPawn_Dodo _asvrpawn_dodo))
    (:then_1
      ;[1 1 1] 箭头旋转
      (bind _returnvalue (Utilities|Time|SetTimerbyEvent (EventDispatchers|CreateEvent :!event Custom|ArrowRotating) (/ 1.0 6e+01) true))
      (Variables|Timers|SetTimer_ArrowRotating _returnvalue))
    (:then_2
      ;[1 1 1] 创建全息引导头盔的动态材质实例
      (bind _returnvalue_2 (Rendering|Material|CreateDynamicMaterialInstance (Variables|Default|GetSM_HoloGuide) 0 0 "None" :!class /Script/Engine.PrimitiveComponent))
      (Variables|DMI|SetDMI_HoloGuide1 _returnvalue_2))))

(fn ConstructionScript)