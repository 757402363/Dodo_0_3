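; Floating robot menu actor that gives VR players touch buttons for standby, movement toggle, calibration level and quitting.
; A 60 Hz timer eases it toward the VR or PC test pawn's standby or UI arrow using the GameInstance interpolation speed.
; Hand overlaps open the UI, while timelines drive dynamic-material opacity and buttons unlock after fade-in.
; Calibration and quit fade the camera to white first, with calibration saving the previous map name.
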(event OnComponentHit(SM_Robot_UI)
  (params (HitComponent :type Primitive%20Component%20Object%20Reference) (OtherActor :type Actor%20Object%20Reference) (OtherComp :type Primitive%20Component%20Object%20Reference) (NormalImpulse :type Vector :default "0, 0, 0") (Hit :type Hit%20Result%20Structure%20%28by%20ref%29))
  ;[1 1 1] 触碰UI机器人，进入UI状态
  ;;[1 1 0] PcPawn测试
)

(event OnComponentBeginOverlap(SphereCollision)
  (params (OverlappedComponent :type Primitive%20Component%20Object%20Reference) (OtherActor :type Actor%20Object%20Reference) (OtherComp :type Primitive%20Component%20Object%20Reference) (OtherBodyIndex :type Integer) (bFromSweep :type Boolean) (SweepResult :type Hit%20Result%20Structure%20%28by%20ref%29))
  ;[1 1 1] 触碰UI机器人，进入UI状态
  (bind _asbp_hand_left (Utilities|Casting|CastToBP_Hand_Left OtherActor)
    (:then
      (Variables|References|SetBP_Hand_Left _asbp_hand_left))
    (:CastFailed
      (bind _asbp_hand_right (Utilities|Casting|CastToBP_Hand_Right OtherActor))
      (Variables|References|SetBP_Hand_Right _asbp_hand_right)))
  (CallFunction|StateUI))

(event OnComponentBeginOverlap(BoxCollision)
  (params (OverlappedComponent :type Primitive%20Component%20Object%20Reference) (OtherActor :type Actor%20Object%20Reference) (OtherComp :type Primitive%20Component%20Object%20Reference) (OtherBodyIndex :type Integer) (bFromSweep :type Boolean) (SweepResult :type Hit%20Result%20Structure%20%28by%20ref%29))
  ;[1 1 1] 触碰UI机器人，进入UI状态
  (bind _asbp_hand_left (Utilities|Casting|CastToBP_Hand_Left OtherActor)
    (:then
      (Variables|References|SetBP_Hand_Left _asbp_hand_left))
    (:CastFailed
      (bind _asbp_hand_right (Utilities|Casting|CastToBP_Hand_Right OtherActor))
      (Variables|References|SetBP_Hand_Right _asbp_hand_right)))
  (CallFunction|StateUI))

(event OnComponentBeginOverlap(Box_Standby)
  (params (OverlappedComponent :type Primitive%20Component%20Object%20Reference) (OtherActor :type Actor%20Object%20Reference) (OtherComp :type Primitive%20Component%20Object%20Reference) (OtherBodyIndex :type Integer) (bFromSweep :type Boolean) (SweepResult :type Hit%20Result%20Structure%20%28by%20ref%29))
  ;[1 1 1] UI_待机模式
  (if (Variables|State|GetBoxAllow)
    (bind _asbp_hand_left (Utilities|Casting|CastToBP_Hand_Left OtherActor)
      (:then
        (Variables|References|SetBP_Hand_Left _asbp_hand_left))
      (:CastFailed
        (bind _asbp_hand_right (Utilities|Casting|CastToBP_Hand_Right OtherActor))
        (Variables|References|SetBP_Hand_Right _asbp_hand_right)))
    (CallFunction|StateStandby)))

(event OnComponentBeginOverlap(Box_Movement)
  (params (OverlappedComponent :type Primitive%20Component%20Object%20Reference) (OtherActor :type Actor%20Object%20Reference) (OtherComp :type Primitive%20Component%20Object%20Reference) (OtherBodyIndex :type Integer) (bFromSweep :type Boolean) (SweepResult :type Hit%20Result%20Structure%20%28by%20ref%29))
  (bind _vrpawn_dodo (Variables|References|GetVRPawn_Dodo))
  ;[1 1 1] UI_移动模式
  (if (Variables|State|GetBoxAllow)
    (bind _asbp_hand_left (Utilities|Casting|CastToBP_Hand_Left OtherActor)
      (:then
        (Variables|References|SetBP_Hand_Left _asbp_hand_left))
      (:CastFailed
        (bind _asbp_hand_right (Utilities|Casting|CastToBP_Hand_Right OtherActor))
        (Variables|References|SetBP_Hand_Right _asbp_hand_right)))
    (if (Variables|State|GetIsStandby)
      _
      (else
        (CallFunction|StateStandby)))
    (Utilities|FlowControl|FlipFlop
      (:A
        (Default|MovementStart _vrpawn_dodo))
      (:B
        (Default|MovementEnd _vrpawn_dodo)))))

(event OnComponentBeginOverlap(Box_Calibration)
  (params (OverlappedComponent :type Primitive%20Component%20Object%20Reference) (OtherActor :type Actor%20Object%20Reference) (OtherComp :type Primitive%20Component%20Object%20Reference) (OtherBodyIndex :type Integer) (bFromSweep :type Boolean) (SweepResult :type Hit%20Result%20Structure%20%28by%20ref%29))
  ;[1 1 1] UI_进入校准
  (if (Variables|State|GetBoxAllow)
    (bind _asbp_hand_left (Utilities|Casting|CastToBP_Hand_Left OtherActor)
      (:then
        (Variables|References|SetBP_Hand_Left _asbp_hand_left))
      (:CastFailed
        (bind _asbp_hand_right (Utilities|Casting|CastToBP_Hand_Right OtherActor))
        (Variables|References|SetBP_Hand_Right _asbp_hand_right)))
    (Variables|State|SetBoxAllow false)
    (CameraFades|StartCameraFade (Game|GetPlayerCameraManager 0) 0.0 1.0 1.5 "(R=1.000000,G=1.000000,B=1.000000,A=1.000000)" false true)
    (Utilities|FlowControl|Delay 1.5)
    (bind _returnvalue (Game|GetCurrentLevelName true))
    (if (Utilities|Enum|NotEqual(Enum) _returnvalue "Map_Calibration_Dodo")
      (Variables|/Game/0_Dodo_0_3/Core/GameInstance_Dodo.GameInstance_Dodo_C|SetNameOfLastMap (Variables|References|GetGameInstance_Dodo) _returnvalue))
    (Game|OpenLevel(byObjectReference) "/Game/0_Dodo_0_3/Maps/Map_Calibration_Dodo.Map_Calibration_Dodo")))

(event OnComponentBeginOverlap(Box_Quit)
  (params (OverlappedComponent :type Primitive%20Component%20Object%20Reference) (OtherActor :type Actor%20Object%20Reference) (OtherComp :type Primitive%20Component%20Object%20Reference) (OtherBodyIndex :type Integer) (bFromSweep :type Boolean) (SweepResult :type Hit%20Result%20Structure%20%28by%20ref%29))
  ;[1 1 1] UI_退出游戏
  (if (Variables|State|GetBoxAllow)
    (bind _asbp_hand_left (Utilities|Casting|CastToBP_Hand_Left OtherActor)
      (:then
        (Variables|References|SetBP_Hand_Left _asbp_hand_left))
      (:CastFailed
        (bind _asbp_hand_right (Utilities|Casting|CastToBP_Hand_Right OtherActor))
        (Variables|References|SetBP_Hand_Right _asbp_hand_right)))
    (Variables|State|SetBoxAllow false)
    (CameraFades|StartCameraFade (Game|GetPlayerCameraManager 0) 0.0 1.0 1.5 "(R=1.000000,G=1.000000,B=1.000000,A=1.000000)" false true)
    (Utilities|FlowControl|Delay 1.5)
    (Development|ExecuteConsoleCommand "quit" 0)))

(event Custom|Transform_Robot_VR
  (bind _vrpawn_dodo (Variables|References|GetVRPawn_Dodo))
  (bind _isstandby (Variables|State|GetIsStandby))
  (bind _vrpawn_dodo_2 (Variables|References|GetVRPawn_Dodo))
  (bind _robot_ui_standby_arrow (Variables|/Game/0_Dodo_0_3/Characters/VRPawn/VRPawn_Dodo.VRPawn_Dodo_C|GetRobot_UI_Standby_Arrow _vrpawn_dodo_2))
  (bind _robot_ui_arrow (Variables|/Game/0_Dodo_0_3/Characters/VRPawn/VRPawn_Dodo.VRPawn_Dodo_C|GetRobot_UI_Arrow _vrpawn_dodo))
  (bind _returnvalue (select _isstandby _robot_ui_standby_arrow _robot_ui_arrow))
  (bind _returnvalue_2 (Transformation|GetWorldTransform _returnvalue))
  ;[1 1 1] （VR）UI机器人跟随变换
  (Transformation|SetActorTransform (Class|KismetMathLibrary|TInterpto (Transformation|GetActorTransform) (Math|Transform|MakeTransform (.location _returnvalue_2) (.rotation _returnvalue_2) "1,1,1") (Utilities|Time|GetWorldDeltaSeconds) (Utilities|Struct|BreakStruc_VRPlayerSettings (Variables|/Game/0_Dodo_0_3/Core/GameInstance_Dodo.GameInstance_Dodo_C|GetStruc_VRPlayerSettings (Variables|References|GetGameInstance_Dodo))))))

(event Custom|State_UI
  ;[1 1 1] UI机器人状态
  (Variables|State|SetIsStandby false)
  (bind _line0 (Timeline|Opacity_UI PlayFromStart)
    (:Update
      (CallFunction|SetOpacityOfUI _line0))
    (:Finished
      (Variables|State|SetBoxAllow true))))

(event Custom|Transform_Robot_PC
  (bind _bpc_pcpawn_character (Variables|References|GetBPc_PCPawn_Character))
  (bind _bpc_pcpawn_character_2 (Variables|References|GetBPc_PCPawn_Character))
  (bind _isstandby (Variables|State|GetIsStandby))
  (bind _robot_ui_standby_arrow (Variables|/Game/0_Dodo_0_3/Characters/PCPawn/BPc_PCPawn_Character.BPc_PCPawn_Character_C|GetRobot_UI_Standby_Arrow _bpc_pcpawn_character_2))
  (bind _robot_ui_arrow (Variables|/Game/0_Dodo_0_3/Characters/PCPawn/BPc_PCPawn_Character.BPc_PCPawn_Character_C|GetRobot_UI_Arrow _bpc_pcpawn_character))
  (bind _returnvalue (select _isstandby _robot_ui_standby_arrow _robot_ui_arrow))
  (bind _returnvalue_2 (Transformation|GetWorldTransform _returnvalue))
  ;[1 1 1] （PC）UI机器人跟随变换
  (Transformation|SetActorTransform (Class|KismetMathLibrary|TInterpto (Transformation|GetActorTransform) (Math|Transform|MakeTransform (.location _returnvalue_2) (.rotation _returnvalue_2) "1,1,1") (Utilities|Time|GetWorldDeltaSeconds) (Utilities|Struct|BreakStruc_VRPlayerSettings (Variables|/Game/0_Dodo_0_3/Core/GameInstance_Dodo.GameInstance_Dodo_C|GetStruc_VRPlayerSettings (Variables|References|GetGameInstance_Dodo))))))

(event Custom|SetOpacityOfUI
  (params (OpacityOfUI :type Float%20%28single-precision%29))
  (bind _sm_quit (Variables|Default|GetSM_Quit))
  (bind _sm_standby (Variables|Default|GetSM_Standby))
  (bind _sm_movement (Variables|Default|GetSM_Movement))
  (bind _sm_calibration (Variables|Default|GetSM_Calibration))
  ;[1 1 1] 设置UI的动态材质实例（不透明度）
  (Variables|UI|SetOpacityOfUI OpacityOfUI)
  (Utilities|FlowControl|Sequence
    (:then_0
      ;;[0 0 0] 动态材质实例_不透明度（待机模式）
      (Utilities|FlowControl|Sequence
        (:then_0
          (Utilities|IsValid (Variables|UI|GetDMI_Standby_0)
            (:Is%20Valid
              _)
            (:Is%20Not%20Valid
              (bind _returnvalue (Rendering|Material|CreateDynamicMaterialInstance _sm_standby 0 0 "None" :!class /Script/Engine.PrimitiveComponent))
              (Variables|UI|SetDMI_Standby_0 _returnvalue)))
          (Rendering|Material|SetScalarParameterValue (Variables|UI|GetDMI_Standby_0) "Opacity" (Variables|UI|GetOpacityOfUI) :!class /Script/Engine.MaterialInstanceDynamic))
        (:then_1
          (Utilities|IsValid (Variables|UI|GetDMI_Standby_1)
            (:Is%20Valid
              _)
            (:Is%20Not%20Valid
              (bind _returnvalue_2 (Rendering|Material|CreateDynamicMaterialInstance _sm_standby 1 0 "None" :!class /Script/Engine.PrimitiveComponent))
              (Variables|UI|SetDMI_Standby_1 _returnvalue_2)))
          (Rendering|Material|SetScalarParameterValue (Variables|UI|GetDMI_Standby_1) "Opacity" (Variables|UI|GetOpacityOfUI) :!class /Script/Engine.MaterialInstanceDynamic))))
    (:then_1
      ;;[0 0 0] 动态材质实例_不透明度（移动控制）
      (Utilities|FlowControl|Sequence
        (:then_0
          (Utilities|IsValid (Variables|UI|GetDMI_Movement_0)
            (:Is%20Valid
              _)
            (:Is%20Not%20Valid
              (bind _returnvalue_3 (Rendering|Material|CreateDynamicMaterialInstance _sm_movement 0 0 "None" :!class /Script/Engine.PrimitiveComponent))
              (Variables|UI|SetDMI_Movement_0 _returnvalue_3)))
          (Rendering|Material|SetScalarParameterValue (Variables|UI|GetDMI_Movement_0) "Opacity" (Variables|UI|GetOpacityOfUI) :!class /Script/Engine.MaterialInstanceDynamic))
        (:then_1
          (Utilities|IsValid (Variables|UI|GetDMI_Movement_1)
            (:Is%20Valid
              _)
            (:Is%20Not%20Valid
              (bind _returnvalue_4 (Rendering|Material|CreateDynamicMaterialInstance _sm_movement 1 0 "None" :!class /Script/Engine.PrimitiveComponent))
              (Variables|UI|SetDMI_Movement_1 _returnvalue_4)))
          (Rendering|Material|SetScalarParameterValue (Variables|UI|GetDMI_Movement_1) "Opacity" (Variables|UI|GetOpacityOfUI) :!class /Script/Engine.MaterialInstanceDynamic))))
    (:then_2
      ;;[0 0 0] 动态材质实例_不透明度（开始/退出 校准）
      (Utilities|FlowControl|Sequence
        (:then_0
          (Utilities|IsValid (Variables|UI|GetDMI_Calibration_0)
            (:Is%20Valid
              _)
            (:Is%20Not%20Valid
              (bind _returnvalue_5 (Rendering|Material|CreateDynamicMaterialInstance _sm_calibration 0 0 "None" :!class /Script/Engine.PrimitiveComponent))
              (Variables|UI|SetDMI_Calibration_0 _returnvalue_5)))
          (Rendering|Material|SetScalarParameterValue (Variables|UI|GetDMI_Calibration_0) "Opacity" (Variables|UI|GetOpacityOfUI) :!class /Script/Engine.MaterialInstanceDynamic))
        (:then_1
          (Utilities|IsValid (Variables|UI|GetDMI_Calibration_1)
            (:Is%20Valid
              _)
            (:Is%20Not%20Valid
              (bind _returnvalue_6 (Rendering|Material|CreateDynamicMaterialInstance _sm_calibration 1 0 "None" :!class /Script/Engine.PrimitiveComponent))
              (Variables|UI|SetDMI_Calibration_1 _returnvalue_6)))
          (Rendering|Material|SetScalarParameterValue (Variables|UI|GetDMI_Calibration_1) "Opacity" (Variables|UI|GetOpacityOfUI) :!class /Script/Engine.MaterialInstanceDynamic))))
    (:then_3
      ;;[0 0 0] 动态材质实例_不透明度（退出游戏）
      (Utilities|FlowControl|Sequence
        (:then_0
          (Utilities|IsValid (Variables|UI|GetDMI_Quit_0)
            (:Is%20Valid
              _)
            (:Is%20Not%20Valid
              (bind _returnvalue_7 (Rendering|Material|CreateDynamicMaterialInstance _sm_quit 0 0 "None" :!class /Script/Engine.PrimitiveComponent))
              (Variables|UI|SetDMI_Quit_0 _returnvalue_7)))
          (Rendering|Material|SetScalarParameterValue (Variables|UI|GetDMI_Quit_0) "Opacity" (Variables|UI|GetOpacityOfUI) :!class /Script/Engine.MaterialInstanceDynamic))
        (:then_1
          (Utilities|IsValid (Variables|UI|GetDMI_Quit_1)
            (:Is%20Valid
              _)
            (:Is%20Not%20Valid
              (bind _returnvalue_8 (Rendering|Material|CreateDynamicMaterialInstance _sm_quit 1 0 "None" :!class /Script/Engine.PrimitiveComponent))
              (Variables|UI|SetDMI_Quit_1 _returnvalue_8)))
          (Rendering|Material|SetScalarParameterValue (Variables|UI|GetDMI_Quit_1) "Opacity" (Variables|UI|GetOpacityOfUI) :!class /Script/Engine.MaterialInstanceDynamic))))))

(event Custom|State_Standby
  ;[1 1 1] UI机器人状态
  (Variables|State|SetIsStandby true)
  (Variables|State|SetBoxAllow false)
  (bind _line0 (Timeline|Opacity_Standby PlayFromStart)
    (:Update
      (CallFunction|SetOpacityOfUI _line0))))

(event EventBeginPlay
  (bind _returnvalue (/ 1.0 6e+01))
  (Utilities|FlowControl|Sequence
    (:then_0
      ;[1 1 1] 引用游戏实例和VRPawn或PCPawn
      (bind _asgame_instance_dodo (Utilities|Casting|CastToGameInstance_Dodo (Game|GetGameInstance)))
      (Variables|References|SetGameInstance_Dodo _asgame_instance_dodo))
    (:then_1
      (bind _asvrpawn_dodo (Utilities|Casting|CastToVRPawn_Dodo (Game|Player|GetPlayerPawn 0)))
      (Variables|References|SetVRPawn_Dodo _asvrpawn_dodo)
      ;[1 1 1] 调用Pawn成功时设置定时器调用对应跟随变换事件
      (bind _returnvalue_2 (Utilities|Time|SetTimerbyEvent (EventDispatchers|CreateEvent :!event Custom|Transform_Robot_VR) _returnvalue true))
      (Variables|Timers|SetTimer_RobotTransform_VR _returnvalue_2))
    (:then_2
      (bind _asbpc_pcpawn_character (Utilities|Casting|CastToBPc_PCPawn_Character (Game|Player|GetPlayerPawn 0)))
      (Variables|References|SetBPc_PCPawn_Character _asbpc_pcpawn_character)
      ;;[1 1 0] PCPawn测试
      (bind _returnvalue_3 (Utilities|Time|SetTimerbyEvent (EventDispatchers|CreateEvent :!event Custom|Transform_Robot_PC) _returnvalue true))
      (Variables|Timers|SetTimer_RobotTransform_PC _returnvalue_3))
    (:then_3
      ;[1 1 1] 启动时隐藏UI按钮
      (CallFunction|SetOpacityOfUI 0.0))))

(event Input|KeyboardEvents|1
  (params (Key :type Key%20Structure))
  ;[1 1 1] UI_待机模式
  ;;[1 1 0] 仅供PCPawn测试
)

(fn ConstructionScript)