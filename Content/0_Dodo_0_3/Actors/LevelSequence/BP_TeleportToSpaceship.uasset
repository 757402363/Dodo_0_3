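; Trigger actor that plays the teleport-to-spaceship cutscene and then opens the next level (Map_Temp).
; When the VR or PC pawn overlaps the box, it fades to white, hides and unpossesses the pawn, and shows intro UMG text in VR or just waits on PC.
; It then plays the level sequence, triggers the large spaceship's sequence event, fades out its looping BGM and times camera fades with chained delays until the level change.
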(event OnComponentBeginOverlap(Box)
  (params (OverlappedComponent :type Primitive%20Component%20Object%20Reference) (OtherActor :type Actor%20Object%20Reference) (OtherComp :type Primitive%20Component%20Object%20Reference) (OtherBodyIndex :type Integer) (bFromSweep :type Boolean) (SweepResult :type Hit%20Result%20Structure%20%28by%20ref%29))
  ;[1 1 1] 过场动画变化内容
  (bind _asvrpawn_dodo (Utilities|Casting|CastToVRPawn_Dodo OtherActor)
    (:then
      (Variables|References|SetVRPawn_Dodo _asvrpawn_dodo))
    (:CastFailed
      (bind _asbpc_pcpawn_character (Utilities|Casting|CastToBPc_PCPawn_Character OtherActor))
      (Variables|References|SetBPc_PCPawn_Character _asbpc_pcpawn_character)))
  ;;[0 0 0] 屏幕渐白
  (CameraFades|StartCameraFade (Game|GetPlayerCameraManager 0) 0.0 1.0 3.0 "(R=1.000000,G=1.000000,B=1.000000,A=1.000000)" false true)
  (Utilities|FlowControl|Delay 3.0)
  ;;[0 0 0] 隐藏Pawn（避免被过场动画拍到）并解控（避免误触）
  (if (Utilities|IsValid (Variables|References|GetVRPawn_Dodo))
    (Rendering|SetActorHiddenInGame (Variables|References|GetVRPawn_Dodo) true)
    (Pawn|UnPossess (Game|GetPlayerController 0))
    (Components|DestroyComponent (Variables|Default|GetBox))
    ;;[0 0 0] 如果为VRPawn，显示进入过场动画UMG提示
    (bind _line0 (Timeline|ShowUMG_SequenceBegin PlayFromStart)
      (:Update
        (Widget|SetRenderOpacity (Variables|/Game/0_Dodo_0_3/UI/UMG/UMG_State_Dodo.UMG_State_Dodo_C|GetText_State_SequenceBegin_L (Variables|/Game/0_Dodo_0_3/Characters/VRPawn/VRPawn_Dodo.VRPawn_Dodo_C|GetUMG_State_Dodo (Variables|References|GetVRPawn_Dodo))) _line0))
      (:Finished
        ;;[0 0 0] 过场动画
        (bind _outactor (Sequencer|Player|CreateLevelSequencePlayer "/Game/0_Dodo_0_3/Sequences/LSq_ToSpaceship.LSq_ToSpaceship" :!label _label))
        (Sequencer|Player|Play (Variables|/Script/LevelSequence.LevelSequenceActor|GetSequencePlayer _outactor) :!class /Script/MovieScene.MovieSceneSequencePlayer)
        (Default|SequencetoSpaceship (Variables|References|GetSpaceship_large))
        ;;[0 0 0] 进入过场动画，原游戏BGM音量渐小至消失
        (CameraFades|StartCameraFade (Game|GetPlayerCameraManager 0) 1.0 0.0 3.0 "(R=1.000000,G=1.000000,B=1.000000,A=1.000000)" false false)
        (Audio|Components|Audio|AdjustVolume (Variables|Default|GetBGM) 3.0 0.0 "Linear" :!class /Script/Engine.AudioComponent)
        (Utilities|FlowControl|Delay 3.0)
        (Components|DestroyComponent (Variables|Default|GetBGM))
        ;;[0 0 0] 过场动画摄像机切换
        (Utilities|FlowControl|Delay 27.5)
        (CameraFades|StartCameraFade (Game|GetPlayerCameraManager 0) 0.0 1.0 3.0 "(R=1.000000,G=1.000000,B=1.000000,A=1.000000)" true true)
        (Utilities|FlowControl|Delay 3.0)
        (CameraFades|StartCameraFade (Game|GetPlayerCameraManager 0) 1.0 0.0 3.0 "(R=1.000000,G=1.000000,B=1.000000,A=1.000000)" true false)
        ;;[0 0 0] 视野渐黑至过场动画结束，进入下一关卡
        (Utilities|FlowControl|Delay 2e+01)
        (CameraFades|StartCameraFade (Game|GetPlayerCameraManager 0) 0.0 1.0 3.0 "(R=0.000000,G=0.000000,B=0.000000,A=1.000000)" true true)
        (Utilities|FlowControl|Delay 3.0)
        (Sequencer|Player|Stop (Variables|/Script/LevelSequence.LevelSequenceActor|GetSequencePlayer _outactor) :!class /Script/MovieScene.MovieSceneSequencePlayer)
        (Game|OpenLevel(byObjectReference) "/Game/0_Dodo_0_3/Maps/Map_Temp.Map_Temp")))
    (else
      (Rendering|SetActorHiddenInGame (Variables|References|GetBPc_PCPawn_Character) true)
      (Pawn|UnPossess (Game|GetPlayerController 0))
      (Components|DestroyComponent (Variables|Default|GetBox))
      (Utilities|FlowControl|Delay 8.0)
      (goto _label))))

(event OnAudioFinished(BGM)
  (bind _bgm (Variables|Default|GetBGM))
  ;[1 1 1] 背景音乐循环
  (Utilities|IsValid _bgm
    (:Is%20Valid
      (Audio|Components|Audio|Play _bgm 0.0))))

(event EventBeginPlay
  ;[1 1 1] 获取飞船Actor的引用
  (bind _outactors (Actor|GetAllActorsOfClass "/Game/0_Dodo_0_3/Actors/Hologram/BP_SpaceShip_Large.BP_Spaceship_Large_C"))
  (Variables|References|SetSpaceship_large (Utilities|Array|Get(acopy) _outactors)))

(fn ConstructionScript)