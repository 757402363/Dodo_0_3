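; BP_HoloGuide is a wearable VR helmet actor with a spinning arrow prompt that shows until a hand comes near.
; BeginPlay caches the VRPawn_Dodo after a short delay and starts a looping timer that rotates the arrow.
; A left or right hand entering the prompt box stops the timer and destroys the prompt components.
; HoloGuide_Wear disables physics and collision, snaps to the pawn's anchor, and sets the pawn as owner to hide the helmet from its wearer.
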(event OnComponentBeginOverlap(Box_Prompt)
  (params (OverlappedComponent :type Primitive%20Component%20Object%20Reference) (OtherActor :type Actor%20Object%20Reference) (OtherComp :type Primitive%20Component%20Object%20Reference) (OtherBodyIndex :type Integer) (bFromSweep :type Boolean) (SweepResult :type Hit%20Result%20Structure%20%28by%20ref%29))
  ;[1 1 1] 手靠近头盔，提示相关组件销毁
  (Utilities|Casting|CastToBP_Hand_Left OtherActor
    (:then
      _)
    (:CastFailed
      (Utilities|Casting|CastToBP_Hand_Right OtherActor)))
  (Utilities|Time|ClearandInvalidateTimerbyHandle (Variables|Timers|GetTimer_ArrowRotating))
  (Components|DestroyComponent (Variables|Default|GetBox_Prompt)))

(event Custom|ArrowRotating
  ;[1 1 1] 箭头旋转
  (Transformation|AddLocalRotation (Variables|Default|GetSM_Arrow_Prompt) "2.000000, 0, 0" false false))

(event Custom|HoloGuide_Wear
  (bind _sm_hologuide (Variables|Default|GetSM_HoloGuide))
  ;[0 0 0] 取消模拟物理与碰撞，将头盔附加到VRPawn的对应箭头处
  (Physics|SetSimulatePhysics _sm_hologuide false)
  (Collision|SetCollisionEnabled _sm_hologuide "NoCollision")
  (Transformation|AttachComponentToComponent (Variables|/Game/0_Dodo_0_3/Characters/VRPawn/VRPawn_Dodo.VRPawn_Dodo_C|GetArrow_HoloGuide (Variables|References|GetVRPawn_Dodo)) "None" "SnapToTarget" "SnapToTarget" "SnapToTarget" true)
  ;[0 0 0] 设置VRPawn为该Actor的拥有者，使头盔能对VRPawn设置拥有者不可见。
  (Actor|SetOwner (Variables|References|GetVRPawn_Dodo))
  (Class|PrimitiveComponent|SetOwnerNoSee (Variables|Default|GetSM_HoloGuide) true))

(event EventBeginPlay
  (Utilities|FlowControl|Sequence
    (:then_0
      ;[1 1 1] 获取VRPawn引用
      (Utilities|FlowControl|Delay 0.1)
      (bind _asvrpawn_dodo (Utilities|Casting|CastToVRPawn_Dodo (Game|Player|GetPlayerPawn 0)))
      (Variables|References|SetVRPawn_Dodo _asvrpawn_dodo))
    (:then_1
      ;[1 1 1] 箭头旋转
      (bind _returnvalue (Utilities|Time|SetTimerbyEvent (EventDispatchers|CreateEvent :!event Custom|ArrowRotating) (/ 1.0 6e+01) true))
      (Variables|Timers|SetTimer_ArrowRotating _returnvalue))))

(fn ConstructionScript)