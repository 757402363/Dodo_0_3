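; BP_Spaceship_Egg is a spaceship actor, filed under Eggs, that flies along world Y with particle effects and space audio.
; BeginPlay reveals the power and yaw thruster components after a brief delay, then two seconds in starts the sound and a looping 60 Hz timer.
; The timer drives movement by a fixed per-tick offset, independent of frame delta, with no stop condition.
; The sound replays whenever it finishes.
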(event OnAudioFinished(Cue_Space)
  ;[1 1 1] 音效循环
  (Audio|Components|Audio|Play (Variables|Default|GetCue_Space) 0.0))

(event Custom|SpaceshipMove
  ;[1 1 1] 飞船移动
  (Transformation|AddActorWorldOffset (Math|Vector|MakeVector 0.0 5e+01 0.0)))

(event EventBeginPlay
  ;[1 1 1] 显示粒子特效，延迟2s播放太空音效，飞船开始移动
  (Utilities|FlowControl|Sequence
    (:then_0
      (Utilities|FlowControl|Delay 0.1)
      (Development|SetHiddeninGame (Variables|Default|GetP_Power1) false false))
    (:then_1
      (Utilities|FlowControl|Delay 2.0)
      (Audio|Components|Audio|Play (Variables|Default|GetCue_Space) 0.0)
      (Utilities|Time|SetTimerbyEvent (EventDispatchers|CreateEvent :!event Custom|SpaceshipMove) (/ 1.0 6e+01) true))))

(fn ConstructionScript)