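; Easter egg actor that sends the player to the hidden space egg level, Map_SpaceScene_Egg.
; On BeginPlay it grabs the BGM component from the level's BP_TeleportToSpaceship.
; The Egg_ToSpace event disables the sphere's physics and collision, then scales it via a timeline while fading the camera to black and the music to silence.
; When the timeline finishes, it opens the egg level.
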(event Custom|Egg_ToSpace
  (bind _sm_egg_tospace (Variables|Default|GetSM_Egg_ToSpace))
  ;[1 1 1] 进入彩蛋关卡前，彩蛋球体取消模拟物理和碰撞且逐渐变大，视野渐黑，BGM音量渐小
  (Physics|SetSimulatePhysics _sm_egg_tospace false)
  (Collision|SetCollisionEnabled _sm_egg_tospace "NoCollision")
  (CameraFades|StartCameraFade (Game|GetPlayerCameraManager 0) 0.0 1.0 5.0 "(R=0.000000,G=0.000000,B=0.000000,A=1.000000)" true true)
  (Audio|Components|Audio|AdjustVolume (Variables|Default|GetBGM) 5.0 0.0 "Linear" :!class /Script/Engine.AudioComponent)
  (bind _line0 (Timeline|TimeLine_Egg_ToSpace PlayFromStart)
    (:Update
      (Transformation|SetWorldScale3D (Variables|Default|GetSM_Egg_ToSpace) (Math|Vector|MakeVector _line0 _line0 _line0)))
    (:Finished
      (Game|OpenLevel(byObjectReference) "/Game/0_Dodo_0_3/Maps/Map_SpaceScene_Egg.Map_SpaceScene_Egg"))))

(event EventBeginPlay
  ;[1 1 1] 获取关卡中的BGM组件便于控制
  (bind _outactors (Actor|GetAllActorsOfClass "/Game/0_Dodo_0_3/Actors/LevelSequence/BP_TeleportToSpaceship.BP_TeleportToSpaceship_C"))
  (Variables|Default|SetBGM (Variables|/Game/0_Dodo_0_3/Actors/LevelSequence/BP_TeleportToSpaceship.BP_TeleportToSpaceship_C|GetBGM (Utilities|Array|Get(acopy) _outactors))))

(fn ConstructionScript)