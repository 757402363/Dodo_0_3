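; BP_SpaceShip_Small is a small spaceship actor in the Hologram set that can fade its opacity before removing itself.
; On BeginPlay it creates dynamic material instances for six material slots of the ship mesh and stores them in an array.
; The DestroyActor event plays a timeline that drives the Opacity parameter on each instance, then destroys the actor when the timeline finishes.
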(event Custom|DestroyActor
  ;[1 1 1] 销毁Actor
  (bind _line0 (Timeline|OpacityOfSpaceShip PlayFromStart)
    (:Update
      (for _index (range 0 5)
        (Rendering|Material|SetScalarParameterValue (Utilities|Array|Get(acopy) (Variables|Default|GetDMIs_SpaceShip) _index) "Opacity" _line0 :!class /Script/Engine.MaterialInstanceDynamic)))
    (:Finished
      (Actor|DestroyActor))))

(event EventBeginPlay
  ;[1 1 1] 设置动态材质实例
  (for _index (range 0 5)
    (bind _returnvalue (Rendering|Material|CreateDynamicMaterialInstance (Variables|Default|GetSM_SpaceShip) _index 0 "None" :!class /Script/Engine.PrimitiveComponent))
    (Utilities|Array|Add (Variables|Default|GetDMIs_SpaceShip) _returnvalue)))

(fn ConstructionScript)