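; Interactive hologram of a building, started by a hand or PC pawn touch, that lets a small spaceship be placed into it.
; Timelines fade in dynamic materials and control handles, which become physics-simulated and drive a 60 Hz timer.
; Two handles set scale by distance and yaw by angle; a third sets interpolated position.
; Overlapping the small ship destroys it, turns the dissolve ship holographic, then reveals the large ship and arrows.
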(event OnComponentBeginOverlap(SM_SpaceShip)
  (params (OverlappedComponent :type Primitive%20Component%20Object%20Reference) (OtherActor :type Actor%20Object%20Reference) (OtherComp :type Primitive%20Component%20Object%20Reference) (OtherBodyIndex :type Integer) (bFromSweep :type Boolean) (SweepResult :type Hit%20Result%20Structure%20%28by%20ref%29))
  ;[1 1 1] 飞船模型与全息图相应位置重叠，小的飞船模型隐藏，大的飞船模型和全息图中飞船显现
  (if (Variables|Default|GetShowSpaceShip_Allow)
    (bind _asbp_space_ship_small (Utilities|Casting|CastToBP_SpaceShip_Small OtherActor))
    (bind _output_get (Variables|Default|SetBP_SpaceShip_Small _asbp_space_ship_small))
    (Default|DestroyActor _output_get)
    (Variables|Default|SetShowSpaceShip_Allow false)
    ;;[0 0 0] 隐藏溶解材质
    (bind _line0 (Timeline|Hide%20SpaceShip_Dissolve PlayFromStart)
      (:Update
        (for _index (range 0 5)
          (Rendering|Material|SetScalarParameterValue (Utilities|Array|Get(acopy) (Variables|Default|GetDMIs_SpaceShip_Dissolve) _index) "Dissolve" _line0 :!class /Script/Engine.MaterialInstanceDynamic)))
      (:Finished
        ;;[0 0 0] 创建全息动态材质实例
        (for _index_2 (range 0 5)
          (bind _returnvalue (Rendering|Material|CreateDynamicMaterialInstance (Variables|Default|GetSM_SpaceShip) _index_2 "/Game/0_Dodo_0_3/Materials/M_Hologram/Instances/MI_Hologram_Blank02.MI_Hologram_Blank02" "None" :!class /Script/Engine.PrimitiveComponent))
          (Rendering|Material|SetScalarParameterValue _returnvalue "Opacity" 0.0 :!class /Script/Engine.MaterialInstanceDynamic)
          (Utilities|Array|Add (Variables|Default|GetDMIs_SpaceShip_Hologram) _returnvalue))
        ;;[0 0 0] 显示全息材质
        (bind _line0_2 (Timeline|Show%20SpaceShip_Hologram PlayFromStart)
          (:Update
            (for _index_3 (range 0 5)
              (Rendering|Material|SetScalarParameterValue (Utilities|Array|Get(acopy) (Variables|Default|GetDMIs_SpaceShip_Hologram) _index_3) "Opacity" _line0_2 :!class /Script/Engine.MaterialInstanceDynamic)))
          (:Finished
            ;[1 1 1] 显示大的飞船模型和所有的箭头指示
            (bind _outactors (Actor|GetAllActorsOfClass "/Game/0_Dodo_0_3/Actors/Hologram/BP_SpaceShip_Large.BP_SpaceShip_Large_C"))
            (Rendering|SetActorHiddenInGame (Utilities|Array|Get(acopy) _outactors) false)
            (bind _outactors_2 (Actor|GetAllActorsOfClass "/Game/0_Dodo_0_3/Actors/Hologram/BP_Arrow.BP_Arrow_C"))
            (Variables|Default|SetBP_Arrows _outactors_2)
            (for _index_4 (range 0 (- (Utilities|Array|Length _outactors_2) 1))
              (Default|ShowArrow (Utilities|Array|Get(acopy) (Variables|Default|GetBP_Arrows) _index_4)))))))))

(event OnComponentBeginOverlap(Box_Start)
  (params (OverlappedComponent :type Primitive%20Component%20Object%20Reference) (OtherActor :type Actor%20Object%20Reference) (OtherComp :type Primitive%20Component%20Object%20Reference) (OtherBodyIndex :type Integer) (bFromSweep :type Boolean) (SweepResult :type Hit%20Result%20Structure%20%28by%20ref%29))
  (bind _sm_transform_rs_2 (Variables|Default|GetSM_Transform_RS_2))
  (bind _sm_transform_l (Variables|Default|GetSM_Transform_L))
  (bind _sm_transform_rs_1 (Variables|Default|GetSM_Transform_RS_1))
  ;[1 1 1] 按下全息图启动按钮
  ;;[0 0 0] 当重叠者为手部或PcPawn，销毁Box_Start避免再次触碰
  (Utilities|Casting|CastToBP_Hand_Left OtherActor
    (:then
      _)
    (:CastFailed
      (Utilities|Casting|CastToBP_Hand_Right OtherActor
        (:then
          _)
        (:CastFailed
          (Utilities|Casting|CastToBPc_PCPawn_Character OtherActor)))))
  (Components|DestroyComponent (Variables|Default|GetBox_Start))
  ;;[0 0 0] 显示全息图以及控制球，并开启模拟物理
  (Rendering|SetVisibility (Variables|Default|GetSM_Transform_RS_1) true false)
  (Rendering|SetVisibility (Variables|Default|GetSM_Transform_RS_2) true false)
  (Rendering|SetVisibility (Variables|Default|GetSM_Transform_L) true false)
  (bind (_direction _line0 _line1) (Timeline|ShowHologram PlayFromStart)
    (:Update
      (Utilities|FlowControl|Sequence
        (:then_0
          (for _index (range 0 192)
            (Rendering|Material|SetScalarParameterValue (Utilities|Array|Get(acopy) (Variables|Default|GetDMIs_HologramBuilding) _index) "Opacity" _line0 :!class /Script/Engine.MaterialInstanceDynamic)))
        (:then_1
          (Transformation|SetWorldScale3D (Variables|Default|GetSM_Transform_RS_1) (Math|Vector|MakeVector (/ _line0 2.0) (/ _line0 2.0) (/ _line0 2.0)))
          (Transformation|SetWorldScale3D (Variables|Default|GetSM_Transform_RS_2) (Math|Vector|MakeVector (/ _line0 2.0) (/ _line0 2.0) (/ _line0 2.0)))
          (Transformation|SetWorldScale3D (Variables|Default|GetSM_Transform_L) (Math|Vector|MakeVector (/ _line0 2.0) (/ _line0 2.0) (/ (/ _line0 2.0) 3.0))))
        (:then_2
          (for _index_2 (range 0 5)
            (Rendering|Material|SetScalarParameterValue (Utilities|Array|Get(acopy) (Variables|Default|GetDMIs_SpaceShip_Dissolve) _index_2) "Dissolve" _line1 :!class /Script/Engine.MaterialInstanceDynamic)))))
    (:Finished
      (Collision|SetCollisionEnabled _sm_transform_rs_1 "QueryAndPhysics")
      (Physics|SetSimulatePhysics _sm_transform_rs_1 true)
      (Collision|SetCollisionEnabled _sm_transform_rs_2 "QueryAndPhysics")
      (Physics|SetSimulatePhysics _sm_transform_rs_2 true)
      (Collision|SetCollisionEnabled _sm_transform_l "QueryAndPhysics")
      (Physics|SetSimulatePhysics _sm_transform_l true)
      ;;[0 0 0] 控制球控制全息图变换
      (Utilities|Time|SetTimerbyEvent (EventDispatchers|CreateEvent :!event Custom|SetTransform) (/ 1.0 6e+01) true)
      (Variables|Default|SetShowSpaceShip_Allow true))))

(event Custom|SetTransform
  (bind _sm_transform_rs_1 (Variables|Default|GetSM_Transform_RS_1))
  (bind _sm_transform_rs_2 (Variables|Default|GetSM_Transform_RS_2))
  (bind _sm_transform_rs_1_2 (Variables|Default|GetSM_Transform_RS_1))
  (bind _sm_transform_rs_2_2 (Variables|Default|GetSM_Transform_RS_2))
  (bind _returnvalue (Transformation|GetWorldLocation _sm_transform_rs_2))
  (bind _returnvalue_2 (Transformation|GetWorldLocation _sm_transform_rs_1))
  (bind _returnvalue_3 (Transformation|GetWorldLocation _sm_transform_rs_1_2))
  (bind _returnvalue_4 (Transformation|GetWorldLocation _sm_transform_rs_2_2))
  (bind _returnvalue_5 (Math|Vector|Distance(Vector) _returnvalue_3 _returnvalue_4))
  (bind _returnvalue_6 (- _returnvalue_2 _returnvalue))
  (bind _returnvalue_7 (Math|Float|MapRangeClamped _returnvalue_5 16.0 1e+02 0.0006 0.015))
  ;[1 1 1] 控制球控制全息图变换
  ;;[0 0 0] 缩放
  (Transformation|SetWorldScale3D (Variables|Default|GetSM_Building) (Math|Vector|MakeVector _returnvalue_7 _returnvalue_7 _returnvalue_7))
  ;;[0 0 0] 旋转
  (Transformation|SetWorldRotation (Variables|Default|GetSM_Building) (Math|Rotator|MakeRotator 0.0 0.0 (Class|KismetMathLibrary|DegAtan2 (.y _returnvalue_6) (.x _returnvalue_6))) false false)
  ;;[0 0 0] 位置
  (Transformation|SetWorldLocation (Variables|Default|GetSM_Building) (Math|Interpolation|VInterpTo (Transformation|GetWorldLocation (Variables|Default|GetSM_Building)) (+ (Transformation|GetWorldLocation (Variables|Default|GetSM_Transform_L)) "5.000000, 0,10.000000") (Utilities|Time|GetWorldDeltaSeconds) 2.0) false false))

(event EventBeginPlay
  (bind _sm_transform_rs_2 (Variables|Default|GetSM_Transform_RS_2))
  (bind _sm_transform_rs_1 (Variables|Default|GetSM_Transform_RS_1))
  (bind _sm_transform_l (Variables|Default|GetSM_Transform_L))
  ;[1 1 1] 设置动态材质实例与隐藏
  (Utilities|FlowControl|Sequence
    (:then_0
      (for _index (range 0 192)
        (bind _returnvalue (Rendering|Material|CreateDynamicMaterialInstance (Variables|Default|GetSM_Building) _index "/Game/0_Dodo_0_3/Materials/M_Hologram/Instances/MI_Hologram_Blank02.MI_Hologram_Blank02" "None" :!class /Script/Engine.PrimitiveComponent))
        (Rendering|Material|SetScalarParameterValue _returnvalue "Opacity" 0.0 :!class /Script/Engine.MaterialInstanceDynamic)
        (Utilities|Array|Add (Variables|Default|GetDMIs_HologramBuilding) _returnvalue)))
    (:then_1
      (for _index_2 (range 0 5)
        (bind _returnvalue_2 (Rendering|Material|CreateDynamicMaterialInstance (Variables|Default|GetSM_SpaceShip) _index_2 0 "None" :!class /Script/Engine.PrimitiveComponent))
        (Rendering|Material|SetScalarParameterValue _returnvalue_2 "Dissolve" 0.35 :!class /Script/Engine.MaterialInstanceDynamic)
        (Utilities|Array|Add (Variables|Default|GetDMIs_SpaceShip_Dissolve) _returnvalue_2)))
    (:then_2
      (Rendering|SetVisibility _sm_transform_rs_1 false false)
      (Collision|SetCollisionEnabled _sm_transform_rs_1 "NoCollision")
      (Rendering|SetVisibility _sm_transform_rs_2 false false)
      (Collision|SetCollisionEnabled _sm_transform_rs_2 "NoCollision")
      (Rendering|SetVisibility _sm_transform_l false false)
      (Collision|SetCollisionEnabled _sm_transform_l "NoCollision"))))

(fn ConstructionScript)