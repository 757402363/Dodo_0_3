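; A spawner actor that pops out a slime when a left hand, right hand or player character overlaps its cube, acting as a button.
; Each slime spawns just above the actor with random rotation and small random scale, then gets a mostly upward force with random horizontal push on its skeletal mesh.
; The timer-based auto-spawn test is left unconnected, so spawning only happens on overlap.
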(event OnComponentBeginOverlap(Cube)
  (params (OverlappedComponent :type Primitive%20Component%20Object%20Reference) (OtherActor :type Actor%20Object%20Reference) (OtherComp :type Primitive%20Component%20Object%20Reference) (OtherBodyIndex :type Integer) (bFromSweep :type Boolean) (SweepResult :type Hit%20Result%20Structure%20%28by%20ref%29))
  (bind _returnvalue (Math|Random|RandomFloatinRange 0.0 5e+03))
  (bind _returnvalue_2 (Math|Random|RandomFloatinRange -3e+01 3e+01))
  (bind _returnvalue_3 (Math|Random|RandomFloatinRange 0.03 0.15))
  ;[1 1 1] 按下按钮，生成Slime并添加大致向上的作用力，其slime的旋转、缩放以及施加作用力的大小和方向都在一定范围内随机
  (Utilities|Casting|CastToBP_Hand_Left OtherActor
    (:then
      _)
    (:CastFailed
      (Utilities|Casting|CastToBP_Hand_Right OtherActor
        (:then
          _)
        (:CastFailed
          (Utilities|Casting|CastToBPc_PCPawn_Character OtherActor)))))
  (bind _returnvalue_4 (Game|SpawnActorfromClass "/Game/0_Dodo_0_3/Actors/Slime/BP_Slime.BP_Slime_C" (Math|Transform|MakeTransform (+ (Transformation|GetActorLocation) "0, 0,25.000000") (Math|Rotator|MakeRotator _returnvalue_2 _returnvalue_2 (Math|Random|RandomFloatinRange 5e+01 1.8e+02)) (Math|Vector|MakeVector _returnvalue_3 _returnvalue_3 _returnvalue_3)) "AdjustIfPossibleButAlwaysSpawn" 0 0))
  (Physics|AddForce (Variables|/Game/0_Dodo_0_3/Actors/Slime/BP_Slime.BP_Slime_C|GetSkM_Slime _returnvalue_4) (Math|Vector|MakeVector _returnvalue _returnvalue 3e+04) "None" false))

(event Custom|Test_SpawnSlime_Auto
  ;[1 1 0] 测试，用于自动生成Slime
)

(event EventBeginPlay
  ;[1 1 0] 测试，用于自动生成Slime
)

(fn ConstructionScript)