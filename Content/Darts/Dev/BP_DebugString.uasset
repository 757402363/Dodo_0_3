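; BP_DebugString is a darts debug actor that displays the dartboard's bonus quadrant and the player's score on a TextRender.
; On BeginPlay it refreshes the text, then binds events to debug dispatchers on GameMode_Darts and BP_Dartboard, apparently for further refreshes.
; Debug finds both actors by class and concatenates the two values with no separator.
; A delayed "Debug" text branch is left unconnected.
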(event Custom|Debug
  (bind _outactors (Actor|GetAllActorsOfClass "/Game/Darts/Core/GameMode_Darts.GameMode_Darts_C"))
  (bind _outactors_2 (Actor|GetAllActorsOfClass "/Game/Darts/Dev/BP_Dartboard.BP_Dartboard_C"))
  (Rendering|Components|TextRender|SetText (Variables|Default|GetTextRender) (Utilities|Text|ToText(String) (Utilities|String|Append (Utilities|String|ToString(Integer) (Variables|/Game/Darts/Dev/BP_Dartboard.BP_Dartboard_C|GetBonusQuadrant (Utilities|Array|Get(acopy) _outactors_2))) "  " (Utilities|String|ToString(Integer) (Variables|/Game/Darts/Core/GameMode_Darts.GameMode_Darts_C|GetPlayerScore (Utilities|Array|Get(acopy) _outactors)))))))

(event EventBeginPlay
  (CallFunction|Debug)
  (bind _outactors (Actor|GetAllActorsOfClass "/Game/Darts/Core/GameMode_Darts.GameMode_Darts_C"))
  (EventDispatchers|BindEventtoDebugString (Utilities|Array|Get(acopy) _outactors) (EventDispatchers|CreateEvent :!event Custom|Debug))
  (bind _outactors_2 (Actor|GetAllActorsOfClass "/Game/Darts/Dev/BP_Dartboard.BP_Dartboard_C"))
  (EventDispatchers|BindEventtoDebugString2 (Utilities|Array|Get(acopy) _outactors_2) (EventDispatchers|CreateEvent :!event Custom|Debug)))

(fn ConstructionScript)