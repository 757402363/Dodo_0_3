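; BP_BGMSender is a grabbable prop in the Darts game whose BGMSender component spins continuously.
; Tick adds a fixed yaw step each frame, independent of delta time and whether the prop is held.
; Pickup disables physics on BGMSender and snaps the root to the "Dart" socket of the supplied component.
; Drop re-enables physics and detaches the actor, keeping its world transform.
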(event EventTick
  (params (DeltaSeconds :type Float%20%28single-precision%29))
  (Transformation|AddWorldRotation (Variables|Default|GetBGMSender) "0,2.000000, 0" false false))

(event EventPickup
  (params (AttachTo :type Scene%20Component%20Object%20Reference))
  (Physics|SetSimulatePhysics (Variables|Default|GetBGMSender) false)
  (Transformation|AttachComponentToComponent (VehicleSound|GetRootComponent) AttachTo "Dart" "SnapToTarget" "SnapToTarget" "KeepWorld" false))

(event EventDrop
  (Physics|SetSimulatePhysics (Variables|Default|GetBGMSender) true)
  (Transformation|DetachFromActor "KeepWorld" "KeepWorld" "KeepWorld"))

(fn ConstructionScript)