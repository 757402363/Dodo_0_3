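; Test Blueprint that produces a timed spark effect from three Arrow components.
; Its LSq event spawns a P_Sparks emitter at each arrow's world location, rotation and scale, with auto-destroy disabled.
; After a fixed delay, the same event destroys all three emitter components.
; The construction script is empty, and nothing in the Blueprint itself calls LSq.
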(event Custom|LSq
  (bind _arrow2 (Variables|Default|GetArrow2))
  (bind _arrow (Variables|Default|GetArrow))
  (bind _arrow1 (Variables|Default|GetArrow1))
  (bind _returnvalue (Transformation|GetWorldTransform _arrow2))
  (bind _returnvalue_2 (Transformation|GetWorldTransform _arrow))
  (bind _returnvalue_3 (Transformation|GetWorldTransform _arrow1))
  (bind _returnvalue_4 (Effects|SpawnEmitteratLocation "/Game/StarterContent/Particles/P_Sparks.P_Sparks" (.location _returnvalue_2) (.rotation _returnvalue_2) (.scale _returnvalue_2) false))
  (bind _returnvalue_5 (Effects|SpawnEmitteratLocation "/Game/StarterContent/Particles/P_Sparks.P_Sparks" (.location _returnvalue_3) (.rotation _returnvalue_3) (.scale _returnvalue_3) false))
  (bind _returnvalue_6 (Effects|SpawnEmitteratLocation "/Game/StarterContent/Particles/P_Sparks.P_Sparks" (.location _returnvalue) (.rotation _returnvalue) (.scale _returnvalue) false))
  (Utilities|FlowControl|Delay 15.0)
  (Components|DestroyComponent _returnvalue_6)
  (Components|DestroyComponent _returnvalue_5)
  (Components|DestroyComponent _returnvalue_4))

(fn ConstructionScript)