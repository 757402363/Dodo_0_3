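; BP_HologramBuilding is a test Blueprint that animates the opacity of a hologram building mesh when play begins.
; On BeginPlay it creates a dynamic instance of MI_Hologram_Blank for each of a hard-coded range of material slots, starts each fully transparent and stores them in an array.
; A timeline then plays from the start, writing its track value to every instance's Opacity parameter on each update.
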(event EventBeginPlay
  (for _index (range 0 192)
    (bind _returnvalue (Rendering|Material|CreateDynamicMaterialInstance (Variables|Default|GetStaticMesh) _index "/Game/0_Dodo_0_3/Materials/M_Hologram/Instances/MI_Hologram_Blank.MI_Hologram_Blank" "None" :!class /Script/Engine.PrimitiveComponent))
    (Rendering|Material|SetScalarParameterValue _returnvalue "Opacity" 0.0 :!class /Script/Engine.MaterialInstanceDynamic)
    (Utilities|Array|Add (Variables|Default|GetNewVar_0) _returnvalue))
  (bind _新建轨道_0 (Timeline|时间轴_0 PlayFromStart)
    (:Update
      (for _index_2 (range 0 192)
        (Rendering|Material|SetScalarParameterValue (Utilities|Array|Get(acopy) (Variables|Default|GetNewVar_0) _index_2) "Opacity" _新建轨道_0 :!class /Script/Engine.MaterialInstanceDynamic)))))

(fn ConstructionScript)