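; Procedural asteroid field actor that scatters randomly placed, rotated and uniformly scaled instances around its origin.
; The construction script loops over AsteroidNumber, adding one instance to each of sixteen Hierarchical Instanced Static Mesh components per pass.
; Distance range, per-axis multipliers and scale settings shape the field; unseeded randomness makes the layout change on every reconstruction.
; The event graph holds only empty stubs, with no gameplay logic.
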(event OnComponentHit(HierarchicalInstancedStaticMesh1)
  (params (HitComponent :type Primitive%20Component%20Object%20Reference) (OtherActor :type Actor%20Object%20Reference) (OtherComp :type Primitive%20Component%20Object%20Reference) (NormalImpulse :type Vector :default "0, 0, 0") (Hit :type Hit%20Result%20Structure%20%28by%20ref%29)))

(event EventBeginPlay)

(event Collision|EventActorBeginOverlap
  (params (OtherActor :type Actor%20Object%20Reference)))

(event EventTick
  (params (DeltaSeconds :type Float%20%28single-precision%29)))

(fn ConstructionScript
  (bind _returnvalue (Math|Random|RandomRotator false))
  (bind _returnvalue_2 (Math|Random|RandomUnitVector))
  (bind _distancemulti_x (Variables|Default|GetDistanceMulti%20X))
  (bind _maximum_scale (Variables|Default|GetMaximum%20Scale))
  (bind _distancemulti_y (Variables|Default|GetDistanceMulti%20Y))
  (bind _distancemulti_z (Variables|Default|GetDistanceMulti%20Z))
  (bind _scale_multiplier (Variables|Default|GetScale%20Multiplier))
  (bind _minimum_distance (Variables|Default|GetMinimum%20Distance))
  (bind _maximum_distance (Variables|Default|GetMaximum%20Distance))
  (bind _minimum_scale (Variables|Default|GetMinimum%20Scale))
  (bind _returnvalue_3 (Math|Random|RandomFloatinRange _minimum_distance _maximum_distance))
  (bind _returnvalue_4 (Math|Random|RandomFloatinRange _minimum_scale _maximum_scale))
  (bind _returnvalue_5 (* (.z _returnvalue_2) _distancemulti_z))
  (bind _returnvalue_6 (* (.x _returnvalue_2) _distancemulti_x))
  (bind _returnvalue_7 (* (.y _returnvalue_2) _distancemulti_y))
  (bind _returnvalue_8 (Math|Vector|MakeVector _returnvalue_6 _returnvalue_7 _returnvalue_5))
  (bind _returnvalue_9 (* _returnvalue_4 _scale_multiplier))
  (bind _returnvalue_10 (* _returnvalue_8 _returnvalue_3))
  (bind _returnvalue_11 (Math|Conversions|ToVector(Float) _returnvalue_9))
  (bind _returnvalue_12 (Math|Transform|MakeTransform _returnvalue_10 _returnvalue _returnvalue_11))
  (for _index (range 0 (Variables|Default|GetAsteroid%20Number))
    (Components|InstancedStaticMesh|AddInstance (Variables|Default|GetHierarchicalInstancedStaticMesh1) _returnvalue_12)
    (Components|InstancedStaticMesh|AddInstance (Variables|Default|GetHierarchicalInstancedStaticMesh2) _returnvalue_12)
    (Components|InstancedStaticMesh|AddInstance (Variables|Default|GetHierarchicalInstancedStaticMesh3) _returnvalue_12)
    (Components|InstancedStaticMesh|AddInstance (Variables|Default|GetHierarchicalInstancedStaticMesh4) _returnvalue_12)
    (Components|InstancedStaticMesh|AddInstance (Variables|Default|GetHierarchicalInstancedStaticMesh5) _returnvalue_12)
    (Components|InstancedStaticMesh|AddInstance (Variables|Default|GetHierarchicalInstancedStaticMesh6) _returnvalue_12)
    (Components|InstancedStaticMesh|AddInstance (Variables|Default|GetHierarchicalInstancedStaticMesh7) _returnvalue_12)
    (Components|InstancedStaticMesh|AddInstance (Variables|Default|GetHierarchicalInstancedStaticMesh8) _returnvalue_12)
    (Components|InstancedStaticMesh|AddInstance (Variables|Default|GetHierarchicalInstancedStaticMesh9) _returnvalue_12)
    (Components|InstancedStaticMesh|AddInstance (Variables|Default|GetHierarchicalInstancedStaticMesh10) _returnvalue_12)
    (Components|InstancedStaticMesh|AddInstance (Variables|Default|GetHierarchicalInstancedStaticMesh11) _returnvalue_12)
    (Components|InstancedStaticMesh|AddInstance (Variables|Default|GetHierarchicalInstancedStaticMesh12) _returnvalue_12)
    (Components|InstancedStaticMesh|AddInstance (Variables|Default|GetHierarchicalInstancedStaticMesh13) _returnvalue_12)
    (Components|InstancedStaticMesh|AddInstance (Variables|Default|GetHierarchicalInstancedStaticMesh14) _returnvalue_12)
    (Components|InstancedStaticMesh|AddInstance (Variables|Default|GetHierarchicalInstancedStaticMesh15) _returnvalue_12)
    (Components|InstancedStaticMesh|AddInstance (Variables|Default|GetHierarchicalInstancedStaticMesh16) _returnvalue_12)))