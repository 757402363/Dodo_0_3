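; Black hole visual actor whose look is driven by a dynamic material on its BlackHole component.
; The construction script creates the material instance and pushes exposed variables into its scalar and vector parameters, covering hole shape, central light, colors, opacity, textures, warp and speed.
; When AlwaysFaceCamera is set, Tick rotates the whole actor toward the player camera, billboard-style, using the look-at rotation from its Arrow component.
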(event EventTick
  (params (DeltaSeconds :type Float%20%28single-precision%29))
  (if (Variables|Default|GetAlways%20face%20camera)
    (Transformation|SetActorRotation (Math|Rotator|FindLookatRotation (Transformation|GetWorldLocation (Variables|Default|GetArrow)) (Transformation|GetWorldLocation (Variables|/Script/Engine.PlayerCameraManager|GetTransformComponent (Game|GetPlayerCameraManager 0)))))))

(fn ConstructionScript
  (bind _black_hole (Variables|Default|GetBlack_Hole))
  (bind _returnvalue (Rendering|Material|CreateDynamicMaterialInstance _black_hole 0 (Rendering|Material|GetMaterial _black_hole 0) "None" :!class /Script/Engine.PrimitiveComponent))
  (Variables|Default|SetDMI_Black_Hole _returnvalue)
  (Utilities|FlowControl|Sequence
    (:then_0
      (if (Variables|Default|GetCentral%20Light/Black%20Hole)
        (Rendering|Material|SetScalarParameterValue (Variables|Default|GetDMI_Black_Hole) "Central Light" 1.0 :!class /Script/Engine.MaterialInstanceDynamic)
        (else
          (Rendering|Material|SetScalarParameterValue (Variables|Default|GetDMI_Black_Hole) "Central Light" 0.0 :!class /Script/Engine.MaterialInstanceDynamic)))
      (Rendering|Material|SetScalarParameterValue (Variables|Default|GetDMI_Black_Hole) "Central Light Intensity" (Variables|Default|GetCentral%20Light%20Intensity) :!class /Script/Engine.MaterialInstanceDynamic)
      (Rendering|Material|SetScalarParameterValue (Variables|Default|GetDMI_Black_Hole) "Global Tile" (Variables|Default|GetGlobal%20Tiling) :!class /Script/Engine.MaterialInstanceDynamic)
      (Rendering|Material|SetScalarParameterValue (Variables|Default|GetDMI_Black_Hole) "Hole Size" (Variables|Default|GetHole%20Size) :!class /Script/Engine.MaterialInstanceDynamic)
      (Rendering|Material|SetScalarParameterValue (Variables|Default|GetDMI_Black_Hole) "Inner/Outer Transition" (Variables|Default|GetInner/Outer%20Transition) :!class /Script/Engine.MaterialInstanceDynamic)
      (Rendering|Material|SetScalarParameterValue (Variables|Default|GetDMI_Black_Hole) "Inner Zone Brightness" (Variables|Default|GetInner%20Zone%20Brightness) :!class /Script/Engine.MaterialInstanceDynamic)
      (Rendering|Material|SetScalarParameterValue (Variables|Default|GetDMI_Black_Hole) "Opacity" (Variables|Default|GetOpacity) :!class /Script/Engine.MaterialInstanceDynamic)
      (Rendering|Material|SetScalarParameterValue (Variables|Default|GetDMI_Black_Hole) "Speed x" (Variables|Default|GetSpeed%20x) :!class /Script/Engine.MaterialInstanceDynamic)
      (Rendering|Material|SetScalarParameterValue (Variables|Default|GetDMI_Black_Hole) "Speed y" (Variables|Default|GetSpeed%20y) :!class /Script/Engine.MaterialInstanceDynamic)
      (Rendering|Material|SetScalarParameterValue (Variables|Default|GetDMI_Black_Hole) "Texture 1" (Variables|Default|GetTexture%201) :!class /Script/Engine.MaterialInstanceDynamic)
      (Rendering|Material|SetScalarParameterValue (Variables|Default|GetDMI_Black_Hole) "Texture 2" (Variables|Default|GetTexture%202) :!class /Script/Engine.MaterialInstanceDynamic)
      (Rendering|Material|SetScalarParameterValue (Variables|Default|GetDMI_Black_Hole) "Texture 3" (Variables|Default|GetTexture%203) :!class /Script/Engine.MaterialInstanceDynamic)
      (Rendering|Material|SetScalarParameterValue (Variables|Default|GetDMI_Black_Hole) "Texture Warp" (Variables|Default|GetTexture%20Warp) :!class /Script/Engine.MaterialInstanceDynamic))
    (:then_1
      (Rendering|Material|SetVectorParameterValue (Variables|Default|GetDMI_Black_Hole) "Inner Color" (Variables|Default|GetInner%20Color) :!class /Script/Engine.MaterialInstanceDynamic)
      (Rendering|Material|SetVectorParameterValue (Variables|Default|GetDMI_Black_Hole) "Outer Color" (Variables|Default|GetOuter%20Color) :!class /Script/Engine.MaterialInstanceDynamic))))