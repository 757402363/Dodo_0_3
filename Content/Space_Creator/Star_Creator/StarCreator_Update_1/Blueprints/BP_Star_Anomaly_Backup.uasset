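; Star anomaly actor that renders a colored star, an animated disk and paired up/down lens flare billboards.
; The construction script pushes editable settings into dynamic materials and sizes the billboards, with optional "Pro" flares.
; Tick traces from camera to star, fading main flare luminosity and interpolating Pro flare luminosity and size on obstruction.
; It also feeds the projected screen position and angle toward screen center into the Pro flare materials.
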(event EventTick
  (params (DeltaSeconds :type Float%20%28single-precision%29))
  (bind _returnvalue (Game|GetPlayerController 0))
  (bind _lensflare_pro_up (Variables|Default|GetLensflare_Pro_Up))
  (bind _dmi_lensflare_pro_up (Variables|Default|GetDMI_Lensflare_Pro_Up))
  (bind _dmi_lensflare_pro_up_2 (Variables|Default|GetDMI_Lensflare_Pro_Up))
  (bind _dmi_lensflare_pro_up_3 (Variables|Default|GetDMI_Lensflare_Pro_Up))
  (bind _returnvalue_2 (Transformation|GetWorldLocation _lensflare_pro_up))
  (bind _screenposition (Class|GameplayStatics|ProjectWorldtoScreen _returnvalue _returnvalue_2 false))
  (bind (_x _y) (Math|Vector2D|BreakVector2D _screenposition))
  (Variables|Default|SetDelta DeltaSeconds)
  (Rendering|Material|SetScalarParameterValue (Variables|Default|GetDMI_lensflare_Main_Up) "Luminosity By Obstacle" (Variables|Default|GetLens%20Luminosity%20By%20Obstancle) :!class /Script/Engine.MaterialInstanceDynamic)
  (bind _returnvalue_3 (Collision|LineTraceByChannel (Transformation|GetWorldLocation (Variables|/Script/Engine.PlayerCameraManager|GetTransformComponent (Game|GetPlayerCameraManager 0))) (Transformation|GetWorldLocation (Variables|Default|GetSphere)) "TraceTypeQuery1" false (Utilities|Array|MakeArray self) "None"))
  (bind _output_get (Variables|Default|SetLensflare%20Visibility _returnvalue_3))
  (if _output_get
    (Variables|Default|SetLens%20Luminosity%20By%20Obstancle (Math|Float|Clamp(Float) (+ (Variables|Default|GetLens%20Luminosity%20By%20Obstancle) -0.06)))
    (else
      (Variables|Default|SetLens%20Luminosity%20By%20Obstancle (Math|Float|Clamp(Float) (+ (Variables|Default|GetLens%20Luminosity%20By%20Obstancle) 0.06)))))
  (if (Variables|Default|GetLensflare%20Visibility)
    (Variables|LensflaresPro|SetLensflare_Pro_Luminosity_NON-EDITABLE (Math|Interpolation|FInterpTo (Variables|LensflaresPro|GetLensflare_Pro_Luminosity_NON-EDITABLE) 0.0 (Variables|Default|GetDelta) (Variables|LensflaresPro|GetFade%20Out%20Speed)))
    (Variables|LensflaresPro|SetSize_Normalized (Math|Interpolation|FInterpTo (Variables|LensflaresPro|GetSize_Normalized) 2e+01 (Variables|Default|GetDelta) (Variables|LensflaresPro|GetFade%20Out%20Speed)))
    (Rendering|Material|SetScalarParameterValue _dmi_lensflare_pro_up_3 "Luminosity" (Math|Interpolation|FInterpTo (Variables|LensflaresPro|GetLensflare_Pro_Luminosity_NON-EDITABLE) 0.0 (Variables|Default|GetDelta) (Variables|LensflaresPro|GetFade%20Out%20Speed)) :!class /Script/Engine.MaterialInstanceDynamic)
    (Rendering|Material|SetScalarParameterValue _dmi_lensflare_pro_up "Size_Normalized" (Math|Interpolation|FInterpTo (Variables|LensflaresPro|GetSize_Normalized) 2e+01 (Variables|Default|GetDelta) (Variables|LensflaresPro|GetFade%20Out%20Speed)) :!class /Script/Engine.MaterialInstanceDynamic)
    (else
      (Variables|LensflaresPro|SetLensflare_Pro_Luminosity_NON-EDITABLE (Math|Interpolation|FInterpTo (Variables|LensflaresPro|GetLensflare_Pro_Luminosity_NON-EDITABLE) 1.0 (Variables|Default|GetDelta) (Variables|LensflaresPro|GetFade%20In%20Speed)))
      (Variables|LensflaresPro|SetSize_Normalized (Math|Interpolation|FInterpTo (Variables|LensflaresPro|GetSize_Normalized) 1.0 (* (Variables|Default|GetDelta) 2.0) (Variables|LensflaresPro|GetFade%20In%20Speed)))
      (Rendering|Material|SetScalarParameterValue _dmi_lensflare_pro_up_3 "Luminosity" (Math|Interpolation|FInterpTo (Variables|LensflaresPro|GetLensflare_Pro_Luminosity_NON-EDITABLE) 1.0 (Variables|Default|GetDelta) (Variables|LensflaresPro|GetFade%20In%20Speed)) :!class /Script/Engine.MaterialInstanceDynamic)
      (Rendering|Material|SetScalarParameterValue _dmi_lensflare_pro_up "Size_Normalized" (Math|Interpolation|FInterpTo (Variables|LensflaresPro|GetSize_Normalized) 1.0 (* (Variables|Default|GetDelta) 2.0) (Variables|LensflaresPro|GetFade%20In%20Speed)) :!class /Script/Engine.MaterialInstanceDynamic)))
  (Rendering|Material|SetScalarParameterValue _dmi_lensflare_pro_up_2 "X" _x :!class /Script/Engine.MaterialInstanceDynamic)
  (Rendering|Material|SetScalarParameterValue _dmi_lensflare_pro_up_2 "Y" _y :!class /Script/Engine.MaterialInstanceDynamic)
  (Rendering|Material|SetScalarParameterValue _dmi_lensflare_pro_up_2 "Angle" (.Yaw (Math|Rotator|BreakRotator (Math|Rotator|FindLookatRotation (Math|Conversions|ToVector(Vector2D) (/ _screenposition (Viewport|GetViewportSize))) (Math|Conversions|ToVector(Vector2D) (/ (/ (Viewport|GetViewportSize) "(X=2.000000,Y=2.000000)") (Viewport|GetViewportSize)))))) :!class /Script/Engine.MaterialInstanceDynamic))

(fn ConstructionScript
  (bind _self self)
  (bind _self_2 self)
  (bind _self_3 self)
  (bind _self_4 self)
  (bind _lensflare_halo_down (Variables|Default|GetLensflare%20Halo_Down))
  (bind _lensflare_halo_up (Variables|Default|GetLensflare%20Halo_Up))
  (bind _lensflare_halo_up_2 (Variables|Default|GetLensflare%20Halo_Up))
  (bind _billboard_size (Variables|LensflaresPro|GetBillboard%20Size))
  (bind _flares_size (Variables|Default|GetFlares%20Size))
  (bind _sphere (Variables|Default|GetSphere))
  (bind _flares_size_2 (Variables|Default|GetFlares%20Size))
  (bind _cube (Variables|Default|GetCube))
  (bind _flares_size_3 (Variables|Default|GetFlares%20Size))
  (bind _flares_size_4 (Variables|Default|GetFlares%20Size))
  (bind _lensflare_main_up (Variables|Default|GetLensflare%20Main_Up))
  (bind _lensflare_main_down (Variables|Default|GetLensflare%20Main_Down))
  (bind _lensflare_main_down_2 (Variables|Default|GetLensflare%20Main_Down))
  (bind _lensflare_main_up_2 (Variables|Default|GetLensflare%20Main_Up))
  (bind _lensflare_pro_up (Variables|Default|GetLensflare_Pro_Up))
  (bind _billboard_size_2 (Variables|LensflaresPro|GetBillboard%20Size))
  (bind _lensflare_pro_up_2 (Variables|Default|GetLensflare_Pro_Up))
  (bind _lensflare_pro_down (Variables|Default|GetLensflare_Pro_Down))
  (bind _lensflare_halo_down_2 (Variables|Default|GetLensflare%20Halo_Down))
  (bind _returnvalue (Transformation|GetActorScale3D _self))
  (bind _returnvalue_2 (Transformation|GetActorScale3D _self_2))
  (bind _returnvalue_3 (Transformation|GetActorScale3D _self_3))
  (bind _returnvalue_4 (Transformation|GetActorScale3D _self_4))
  (bind _returnvalue_5 (* _billboard_size 4.0))
  (bind _returnvalue_6 (* _billboard_size_2 4.0))
  (bind _elements (Variables|/Script/Engine.MaterialBillboardComponent|GetElements _lensflare_halo_down_2))
  (bind _elements_2 (Variables|/Script/Engine.MaterialBillboardComponent|GetElements _lensflare_halo_up))
  (bind _elements_3 (Variables|/Script/Engine.MaterialBillboardComponent|GetElements _lensflare_pro_down))
  (bind _elements_4 (Variables|/Script/Engine.MaterialBillboardComponent|GetElements _lensflare_main_up))
  (bind _elements_5 (Variables|/Script/Engine.MaterialBillboardComponent|GetElements _lensflare_main_down))
  (bind _elements_6 (Variables|/Script/Engine.MaterialBillboardComponent|GetElements _lensflare_pro_up_2))
  (bind _returnvalue_7 (* (.x _returnvalue_4) _flares_size))
  (bind _returnvalue_8 (* (.x _returnvalue_3) _flares_size_3))
  (bind _returnvalue_9 (* (.x _returnvalue_2) _flares_size_2))
  (bind _returnvalue_10 (* (.x _returnvalue) _flares_size_4))
  (bind _output (Utilities|Array|Get(acopy) _elements_3))
  (bind _output_2 (Utilities|Array|Get(acopy) _elements_2))
  (bind _output_3 (Utilities|Array|Get(acopy) _elements_4))
  (bind _output_4 (Utilities|Array|Get(acopy) _elements))
  (bind _output_5 (Utilities|Array|Get(acopy) _elements_5))
  (bind _output_6 (Utilities|Array|Get(acopy) _elements_6))
  (bind (_material _distancetoopacitycurve _bsizeisinscreenspace _basesizex _basesizey _distancetosizecurve) (Utilities|Struct|BreakMaterialSpriteElement _output))
  (bind (_material_2 _distancetoopacitycurve_2 _bsizeisinscreenspace_2 _basesizex_2 _basesizey_2 _distancetosizecurve_2) (Utilities|Struct|BreakMaterialSpriteElement _output_6))
  (bind _returnvalue_11 (Rendering|Material|CreateDynamicMaterialInstance _cube 0 (Rendering|Material|GetMaterial _cube 0) "None" :!class /Script/Engine.PrimitiveComponent))
  (Variables|Default|SetDMI_Disk _returnvalue_11)
  (Utilities|FlowControl|Sequence
    (:then_0
      (Rendering|Material|SetScalarParameterValue (Variables|Default|GetDMI_Disk) "Shadows Offset" (Variables|Default|GetShadows%20Offset) :!class /Script/Engine.MaterialInstanceDynamic)
      (Rendering|Material|SetScalarParameterValue (Variables|Default|GetDMI_Disk) "Shadows Strength" (Variables|Default|GetShadows%20Strength) :!class /Script/Engine.MaterialInstanceDynamic)
      (Rendering|Material|SetScalarParameterValue (Variables|Default|GetDMI_Disk) "Core_Disks_Density" (Variables|Default|GetCore_Disks_Density) :!class /Script/Engine.MaterialInstanceDynamic)
      (Rendering|Material|SetScalarParameterValue (Variables|Default|GetDMI_Disk) "Core_Disks_Radius" (Variables|Default|GetCore_Disks_Radius) :!class /Script/Engine.MaterialInstanceDynamic)
      (Rendering|Material|SetScalarParameterValue (Variables|Default|GetDMI_Disk) "Dense_Clouds_Radius" (Variables|Default|GetDense_Clouds_Radius) :!class /Script/Engine.MaterialInstanceDynamic)
      (Rendering|Material|SetScalarParameterValue (Variables|Default|GetDMI_Disk) "Disk_1_Radius" (Variables|Default|GetDisk_1_Radius) :!class /Script/Engine.MaterialInstanceDynamic)
      (Rendering|Material|SetScalarParameterValue (Variables|Default|GetDMI_Disk) "Disk_2_Radius" (Variables|Default|GetDisk_2_Radius) :!class /Script/Engine.MaterialInstanceDynamic)
      (Rendering|Material|SetScalarParameterValue (Variables|Default|GetDMI_Disk) "Emissive" (Variables|Default|GetEmissive) :!class /Script/Engine.MaterialInstanceDynamic)
      (Rendering|Material|SetScalarParameterValue (Variables|Default|GetDMI_Disk) "Global_Tile" (Variables|Default|GetGlobal_Tile) :!class /Script/Engine.MaterialInstanceDynamic)
      (Rendering|Material|SetScalarParameterValue (Variables|Default|GetDMI_Disk) "Halo" (Variables|Default|GetHalo) :!class /Script/Engine.MaterialInstanceDynamic)
      (Rendering|Material|SetScalarParameterValue (Variables|Default|GetDMI_Disk) "Inner_Disk_Radius" (Variables|Default|GetInner_Disk_Radius) :!class /Script/Engine.MaterialInstanceDynamic)
      (Rendering|Material|SetScalarParameterValue (Variables|Default|GetDMI_Disk) "Opacity" (Variables|Default|GetOpacity) :!class /Script/Engine.MaterialInstanceDynamic)
      (Rendering|Material|SetScalarParameterValue (Variables|Default|GetDMI_Disk) "Opacity_Inner_Density" (Variables|Default|GetOpacity_Inner_Density) :!class /Script/Engine.MaterialInstanceDynamic)
      (Rendering|Material|SetScalarParameterValue (Variables|Default|GetDMI_Disk) "Opacity_Inner_Radius" (Variables|Default|GetOpacity_Inner_Radius) :!class /Script/Engine.MaterialInstanceDynamic)
      (Rendering|Material|SetScalarParameterValue (Variables|Default|GetDMI_Disk) "Opacity_Outer_Density" (Variables|Default|GetOpacity_Outer_Density) :!class /Script/Engine.MaterialInstanceDynamic)
      (Rendering|Material|SetScalarParameterValue (Variables|Default|GetDMI_Disk) "Opacity_Outer_Radius" (Variables|Default|GetOpacity_Outer_Radius) :!class /Script/Engine.MaterialInstanceDynamic)
      (Rendering|Material|SetScalarParameterValue (Variables|Default|GetDMI_Disk) "Outer_Disk_Tile_X" (Variables|Default|GetOuter_Disk_Tile_X) :!class /Script/Engine.MaterialInstanceDynamic)
      (Rendering|Material|SetScalarParameterValue (Variables|Default|GetDMI_Disk) "Outer_Disk_Tile_Y" (Variables|Default|GetOuter_Disk_Tile_Y) :!class /Script/Engine.MaterialInstanceDynamic)
      (Rendering|Material|SetScalarParameterValue (Variables|Default|GetDMI_Disk) "Speed" (Variables|Default|GetSpeed) :!class /Script/Engine.MaterialInstanceDynamic)
      (Rendering|Material|SetScalarParameterValue (Variables|Default|GetDMI_Disk) "Waves_Speed" (Variables|Default|GetWaves_Speed) :!class /Script/Engine.MaterialInstanceDynamic)
      (Rendering|Material|SetScalarParameterValue (Variables|Default|GetDMI_Disk) "Waves_Strength" (Variables|Default|GetWaves_Strength) :!class /Script/Engine.MaterialInstanceDynamic))
    (:then_1
      (Rendering|Material|SetVectorParameterValue (Variables|Default|GetDMI_Disk) "Disk_1_Color" (Variables|Default|GetDisk_1_Color) :!class /Script/Engine.MaterialInstanceDynamic)
      (Rendering|Material|SetVectorParameterValue (Variables|Default|GetDMI_Disk) "Disk_2_Color" (Variables|Default|GetDisk_2_Color) :!class /Script/Engine.MaterialInstanceDynamic)
      (Rendering|Material|SetVectorParameterValue (Variables|Default|GetDMI_Disk) "Disk_3_Color" (Variables|Default|GetDisk_3_Color) :!class /Script/Engine.MaterialInstanceDynamic)
      (Rendering|Material|SetVectorParameterValue (Variables|Default|GetDMI_Disk) "Halo_Color" (Variables|Default|GetHalo_Color) :!class /Script/Engine.MaterialInstanceDynamic)
      (Rendering|Material|SetVectorParameterValue (Variables|Default|GetDMI_Disk) "Inner_Disk_Color" (Variables|Default|GetInner_Disk_Color) :!class /Script/Engine.MaterialInstanceDynamic)
      (Rendering|Material|SetVectorParameterValue (Variables|Default|GetDMI_Disk) "Outer_Color" (Variables|Default|GetOuter_Color) :!class /Script/Engine.MaterialInstanceDynamic))
    (:then_2
      (bind _returnvalue_12 (Rendering|Material|CreateDynamicMaterialInstance _sphere 0 (Rendering|Material|GetMaterial _sphere 0) "None" :!class /Script/Engine.PrimitiveComponent))
      (Rendering|Material|SetVectorParameterValue _returnvalue_12 "Color" (Variables|Default|GetStar_Color) :!class /Script/Engine.MaterialInstanceDynamic)
      (Rendering|Material|SetScalarParameterValue _returnvalue_12 "Lumoinosity" (Variables|Default|GetStar_Luminosity) :!class /Script/Engine.MaterialInstanceDynamic))
    (:then_3
      ;[1 1 1] Lensflares Up
      (Utilities|Array|SetArrayElem _elements_4 0 (Utilities|Struct|MakeMaterialSpriteElement (.material _output_3) 0 false (* (.basesizex _output_3) _returnvalue_10) (* (.basesizey _output_3) _returnvalue_10) (.distancetosizecurve _output_3)))
      (bind _returnvalue_13 (Rendering|Material|CreateDynamicMaterialInstance _lensflare_main_up_2 0 (Rendering|Material|GetMaterial _lensflare_main_up_2 0) "None" :!class /Script/Engine.PrimitiveComponent))
      (Variables|Default|SetDMI_lensflare_Main_Up _returnvalue_13)
      (Rendering|Material|SetVectorParameterValue (Variables|Default|GetDMI_lensflare_Main_Up) "Color" (Variables|Default|GetStar_Color) :!class /Script/Engine.MaterialInstanceDynamic)
      (Utilities|Array|SetArrayElem _elements_2 0 (Utilities|Struct|MakeMaterialSpriteElement (.material _output_2) 0 false (* (.basesizex _output_2) _returnvalue_7) (* (.basesizey _output_2) _returnvalue_7) (.distancetosizecurve _output_2)))
      (bind _returnvalue_14 (Rendering|Material|CreateDynamicMaterialInstance _lensflare_halo_up_2 0 (Rendering|Material|GetMaterial _lensflare_halo_up_2 0) "None" :!class /Script/Engine.PrimitiveComponent))
      (Variables|Default|SetDMI_lensflare_Halo _returnvalue_14)
      (Rendering|Material|SetVectorParameterValue (Variables|Default|GetDMI_lensflare_Halo) "Color" (Variables|Default|GetStar_Color) :!class /Script/Engine.MaterialInstanceDynamic)
      (Rendering|Material|SetScalarParameterValue (Variables|Default|GetDMI_lensflare_Main_Up) "Luminosity" (Variables|Default|GetLensflare%20Luminosity) :!class /Script/Engine.MaterialInstanceDynamic)
      (Rendering|Material|SetScalarParameterValue (Variables|Default|GetDMI_lensflare_Halo) "Luminosity" (Variables|Default|GetHalo%20Flare%20Luminosity) :!class /Script/Engine.MaterialInstanceDynamic))
    (:then_4
      ;[1 1 1] Lensflares Down
      (Utilities|Array|SetArrayElem _elements_5 0 (Utilities|Struct|MakeMaterialSpriteElement (.material _output_5) 0 false (* (.basesizex _output_5) _returnvalue_8) (* (.basesizey _output_5) _returnvalue_8) (.distancetosizecurve _output_5)))
      (bind _returnvalue_15 (Rendering|Material|CreateDynamicMaterialInstance _lensflare_main_down_2 0 (Rendering|Material|GetMaterial _lensflare_main_down_2 0) "None" :!class /Script/Engine.PrimitiveComponent))
      (Variables|Default|SetDMI_lensflare_Main_Down _returnvalue_15)
      (Rendering|Material|SetVectorParameterValue (Variables|Default|GetDMI_lensflare_Main_Down) "Color" (Variables|Default|GetStar_Color) :!class /Script/Engine.MaterialInstanceDynamic)
      (Utilities|Array|SetArrayElem _elements 0 (Utilities|Struct|MakeMaterialSpriteElement (.material _output_4) 0 false (* (.basesizex _output_4) _returnvalue_9) (* (.basesizey _output_4) _returnvalue_9) (.distancetosizecurve _output_4)))
      (bind _returnvalue_16 (Rendering|Material|CreateDynamicMaterialInstance _lensflare_halo_down 0 (Rendering|Material|GetMaterial _lensflare_halo_down 0) "None" :!class /Script/Engine.PrimitiveComponent))
      (Variables|Default|SetDMI_lensflare_Halo _returnvalue_16)
      (Rendering|Material|SetVectorParameterValue (Variables|Default|GetDMI_lensflare_Halo) "Color" (Variables|Default|GetStar_Color) :!class /Script/Engine.MaterialInstanceDynamic)
      (Rendering|Material|SetScalarParameterValue (Variables|Default|GetDMI_lensflare_Main_Down) "Luminosity" (Variables|Default|GetLensflare%20Luminosity) :!class /Script/Engine.MaterialInstanceDynamic)
      (Rendering|Material|SetScalarParameterValue (Variables|Default|GetDMI_lensflare_Halo) "Luminosity" (Variables|Default|GetHalo%20Flare%20Luminosity) :!class /Script/Engine.MaterialInstanceDynamic))
    (:then_5
      ;[1 1 1] Lensflares Pro Integration
      (if (Variables|LensflaresPro|GetEnable%20Lensflares%20Pro)
        (Rendering|SetVisibility _lensflare_pro_up true false)
        (else
          (Rendering|SetVisibility _lensflare_pro_up false false)))
      (bind _returnvalue_17 (Rendering|Material|CreateDynamicMaterialInstance (Variables|Default|GetLensflare_Pro_Up) 0 (Variables|LensflaresPro|GetLensflare_Material) "None" :!class /Script/Engine.PrimitiveComponent))
      (Variables|Default|SetDMI_Lensflare_Pro_Up _returnvalue_17)
      (bind _returnvalue_18 (Rendering|Material|CreateDynamicMaterialInstance (Variables|Default|GetLensflare_Pro_Down) 0 (Variables|LensflaresPro|GetLensflare_Material) "None" :!class /Script/Engine.PrimitiveComponent))
      (Variables|Default|SetDMI_Lensflare_Pro_Down _returnvalue_18)
      (Class|MaterialBillboardComponent|SetElements (Variables|Default|GetLensflare_Pro_Up) (Utilities|Array|MakeArray (Utilities|Struct|MakeMaterialSpriteElement _material_2 _distancetoopacitycurve_2 _bsizeisinscreenspace_2 _returnvalue_6 _returnvalue_6 _distancetosizecurve_2)))
      (Class|MaterialBillboardComponent|SetElements (Variables|Default|GetLensflare_Pro_Down) (Utilities|Array|MakeArray (Utilities|Struct|MakeMaterialSpriteElement _material _distancetoopacitycurve _bsizeisinscreenspace _returnvalue_5 _returnvalue_5 _distancetosizecurve)))
      (if (Variables|LensflaresPro|GetSwitch%20Axis)
        (Rendering|Material|SetScalarParameterValue (Variables|Default|GetDMI_Lensflare_Pro_Up) "Axis" 1.0 :!class /Script/Engine.MaterialInstanceDynamic)
        (else
          (Rendering|Material|SetScalarParameterValue (Variables|Default|GetDMI_Lensflare_Pro_Up) "Axis" 0.0 :!class /Script/Engine.MaterialInstanceDynamic)))
      (Rendering|Material|SetScalarParameterValue (Variables|Default|GetDMI_Lensflare_Pro_Up) "Intensity" (Variables|LensflaresPro|GetIntensity) :!class /Script/Engine.MaterialInstanceDynamic)
      (Rendering|Material|SetScalarParameterValue (Variables|Default|GetDMI_Lensflare_Pro_Up) "Proximity_Ray_Intensity" (Variables|LensflaresPro|GetProximity%20Ray%20Intensity) :!class /Script/Engine.MaterialInstanceDynamic))))