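; Black hole actor from the Star Creator space kit, rendered through a material on its BlackHole component.
; The construction script creates a dynamic material instance and pushes exposed settings for halo, rays, waves, warp, opacity and gas colors into it.
; Every tick it turns the whole actor toward the player camera, measured from an Arrow component, so the effect always faces the view like a billboard.
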(event EventTick
  (params (DeltaSeconds :type Float%20%28single-precision%29))
  (Transformation|SetActorRotation (Math|Rotator|FindLookatRotation (Transformation|GetWorldLocation (Variables|Default|GetArrow self)) (Transformation|GetWorldLocation (Variables|/Script/Engine.PlayerCameraManager|GetTransformComponent (Game|GetPlayerCameraManager 0))))))

(fn ConstructionScript
  (bind _black_hole (Variables|Default|GetBlack_Hole))
  (bind _returnvalue (Rendering|Material|CreateDynamicMaterialInstance _black_hole 0 (Rendering|Material|GetMaterial _black_hole 0) "None" :!class /Script/Engine.PrimitiveComponent))
  (Variables|Default|SetDMI_Black_Hole _returnvalue)
  (Utilities|FlowControl|Sequence
    (:then_0
      (Rendering|Material|SetScalarParameterValue (Variables|Default|GetDMI_Black_Hole) "Halo_Intensity" (Variables|Default|GetHalo_Intensity) :!class /Script/Engine.MaterialInstanceDynamic)
      (Rendering|Material|SetScalarParameterValue (Variables|Default|GetDMI_Black_Hole) "Halo_Warp" (Variables|Default|GetHalo_Warp) :!class /Script/Engine.MaterialInstanceDynamic)
      (Rendering|Material|SetScalarParameterValue (Variables|Default|GetDMI_Black_Hole) "Opacity_Falloff" (Variables|Default|GetOpacity_Falloff) :!class /Script/Engine.MaterialInstanceDynamic)
      (Rendering|Material|SetScalarParameterValue (Variables|Default|GetDMI_Black_Hole) "Rays_Intensity" (Variables|Default|GetRays_Intensity) :!class /Script/Engine.MaterialInstanceDynamic)
      (Rendering|Material|SetScalarParameterValue (Variables|Default|GetDMI_Black_Hole) "Rays_Speed_X" (Variables|Default|GetRays_Speed_X) :!class /Script/Engine.MaterialInstanceDynamic)
      (Rendering|Material|SetScalarParameterValue (Variables|Default|GetDMI_Black_Hole) "Rays_Speed_Y" (Variables|Default|GetRays_Speed_Y) :!class /Script/Engine.MaterialInstanceDynamic)
      (Rendering|Material|SetScalarParameterValue (Variables|Default|GetDMI_Black_Hole) "Rays_Tile" (Variables|Default|GetRays_Tile) :!class /Script/Engine.MaterialInstanceDynamic)
      (Rendering|Material|SetScalarParameterValue (Variables|Default|GetDMI_Black_Hole) "Warp_Amount" (Variables|Default|GetWaves_Warp_Amount) :!class /Script/Engine.MaterialInstanceDynamic)
      (Rendering|Material|SetScalarParameterValue (Variables|Default|GetDMI_Black_Hole) "Waves_Count" (Variables|Default|GetWaves_Count) :!class /Script/Engine.MaterialInstanceDynamic)
      (Rendering|Material|SetScalarParameterValue (Variables|Default|GetDMI_Black_Hole) "Waves_Speed" (Variables|Default|GetWaves_Speed) :!class /Script/Engine.MaterialInstanceDynamic))
    (:then_1
      (Rendering|Material|SetVectorParameterValue (Variables|Default|GetDMI_Black_Hole) "Disk_Gas_Color" (Variables|Default|GetDisk_Gas_Color) :!class /Script/Engine.MaterialInstanceDynamic)
      (Rendering|Material|SetVectorParameterValue (Variables|Default|GetDMI_Black_Hole) "Halo_Color" (Variables|Default|GetHalo_Color) :!class /Script/Engine.MaterialInstanceDynamic)
      (Rendering|Material|SetVectorParameterValue (Variables|Default|GetDMI_Black_Hole) "Inner_Gas_Color" (Variables|Default|GetInner_Gas_Color) :!class /Script/Engine.MaterialInstanceDynamic)
      (Rendering|Material|SetVectorParameterValue (Variables|Default|GetDMI_Black_Hole) "Rays_Color" (Variables|Default|GetRays_Color) :!class /Script/Engine.MaterialInstanceDynamic))))