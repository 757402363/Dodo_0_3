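; Configurable main-sequence star actor with a shader-driven surface, ray particles and a screen-space lens flare.
; Construction script pushes exposed colors, intensities and textures into dynamic materials, and BeginPlay repeats this for surface and rays.
; Tick feeds the lens's projected screen position into its material and fades flare brightness and size whenever a camera-to-star object trace hits.
; Tick also calls CreateDynamicMaterialInstance on the lens every frame rather than caching it.
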(event EventTick
  (params (DeltaSeconds :type Float%20%28single-precision%29))
  (bind _returnvalue (Game|GetPlayerController 0))
  (bind _lens_size (Variables|Default|GetLens_Size))
  (bind _lens (Variables|Default|GetLens))
  (bind _lens_2 (Variables|Default|GetLens))
  (bind _returnvalue_2 (Transformation|GetWorldLocation _lens))
  (bind _screenposition (Class|GameplayStatics|ProjectWorldtoScreen _returnvalue _returnvalue_2 false))
  (bind _returnvalue_3 (Rendering|Material|CreateDynamicMaterialInstance _lens_2 0 (Rendering|Material|GetMaterial _lens_2 0) "None" :!class /Script/Engine.PrimitiveComponent))
  (Rendering|Material|SetScalarParameterValue _returnvalue_3 "Screen_Position" (/ (.x _screenposition) 1e+03) :!class /Script/Engine.MaterialInstanceDynamic)
  (Rendering|Material|SetScalarParameterValue _returnvalue_3 "Screen_Y" (/ (.y _screenposition) 1e+03) :!class /Script/Engine.MaterialInstanceDynamic)
  (Rendering|Material|SetScalarParameterValue _returnvalue_3 "Brightness" (Variables|Default|GetLens_Brightness) :!class /Script/Engine.MaterialInstanceDynamic)
  (Rendering|Material|SetScalarParameterValue _returnvalue_3 "Size" (Variables|Default|GetLens_SizeOnAttenuation) :!class /Script/Engine.MaterialInstanceDynamic)
  (bind _returnvalue_4 (Collision|LineTraceForObjects (Transformation|GetWorldLocation (Variables|/Script/Engine.PlayerCameraManager|GetTransformComponent (Game|GetPlayerCameraManager 0))) (Transformation|GetWorldLocation (Variables|Default|GetStaticMesh)) (Variables|Default|GetObject_Type) false 0 "None"))
  (if _returnvalue_4
    (Variables|Default|SetLens_Brightness (Math|Float|Clamp(Float) (+ (Variables|Default|GetLens_Brightness) -0.05)))
    (Variables|Default|SetLens_SizeOnAttenuation (Math|Float|Clamp(Float) (Math|Float|Clamp(Float) (+ (Variables|Default|GetLens_Brightness) -0.05)) 0.0 _lens_size))
    (else
      (Variables|Default|SetLens_Brightness (Math|Float|Clamp(Float) (+ (Variables|Default|GetLens_Brightness) 0.05)))
      (Variables|Default|SetLens_SizeOnAttenuation (Math|Float|Clamp(Float) (Math|Float|Clamp(Float) (+ (Variables|Default|GetLens_Brightness) 0.05)) 0.0 _lens_size)))))

(event EventBeginPlay
  (bind _main_particle (Variables|Default|GetMain_Particle))
  (bind _main_particle_2 (Variables|Default|GetMain_Particle))
  (bind _main_particle_3 (Variables|Default|GetMain_Particle))
  (bind _main_particle_4 (Variables|Default|GetMain_Particle))
  (bind _staticmesh (Variables|Default|GetStaticMesh))
  (bind _atmosphere_color (Variables|Default|GetAtmosphere_Color))
  (Utilities|FlowControl|Sequence
    (:then_0
      (bind _returnvalue (Rendering|Material|CreateDynamicMaterialInstance _main_particle 0 (Rendering|Material|GetMaterial _main_particle 0) "None" :!class /Script/Engine.PrimitiveComponent))
      (Variables|Default|SetDMI_Main_0 _returnvalue)
      (Rendering|Material|SetScalarParameterValue (Variables|Default|GetDMI_Main_0) "Opacity" (Variables|Default|GetRays_1) :!class /Script/Engine.MaterialInstanceDynamic)
      (Rendering|Material|SetVectorParameterValue (Variables|Default|GetDMI_Main_0) "Color" _atmosphere_color :!class /Script/Engine.MaterialInstanceDynamic))
    (:then_1
      (bind _returnvalue_2 (Rendering|Material|CreateDynamicMaterialInstance _main_particle_2 1 (Rendering|Material|GetMaterial _main_particle_2 1) "None" :!class /Script/Engine.PrimitiveComponent))
      (Variables|Default|SetDMI_Main_1 _returnvalue_2)
      (Rendering|Material|SetScalarParameterValue (Variables|Default|GetDMI_Main_1) "Opacity" (Variables|Default|GetRays_2) :!class /Script/Engine.MaterialInstanceDynamic)
      (Rendering|Material|SetVectorParameterValue (Variables|Default|GetDMI_Main_1) "Color" _atmosphere_color :!class /Script/Engine.MaterialInstanceDynamic))
    (:then_2
      (bind _returnvalue_3 (Rendering|Material|CreateDynamicMaterialInstance _main_particle_3 2 (Rendering|Material|GetMaterial _main_particle_3 2) "None" :!class /Script/Engine.PrimitiveComponent))
      (Variables|Default|SetDMI_Main_2 _returnvalue_3)
      (Rendering|Material|SetScalarParameterValue (Variables|Default|GetDMI_Main_2) "Opacity" (Variables|Default|GetRays_3) :!class /Script/Engine.MaterialInstanceDynamic)
      (Rendering|Material|SetVectorParameterValue (Variables|Default|GetDMI_Main_2) "Color" _atmosphere_color :!class /Script/Engine.MaterialInstanceDynamic))
    (:then_3
      (bind _returnvalue_4 (Rendering|Material|CreateDynamicMaterialInstance _main_particle_4 3 (Rendering|Material|GetMaterial _main_particle_4 3) "None" :!class /Script/Engine.PrimitiveComponent))
      (Variables|Default|SetDMI_Main_3 _returnvalue_4)
      (Rendering|Material|SetScalarParameterValue (Variables|Default|GetDMI_Main_3) "Opacity" (Variables|Default|GetRays_4) :!class /Script/Engine.MaterialInstanceDynamic)
      (Rendering|Material|SetVectorParameterValue (Variables|Default|GetDMI_Main_3) "Color" _atmosphere_color :!class /Script/Engine.MaterialInstanceDynamic))
    (:then_4
      (bind _returnvalue_5 (Rendering|Material|CreateDynamicMaterialInstance _staticmesh 0 (Rendering|Material|GetMaterial _staticmesh 0) "None" :!class /Script/Engine.PrimitiveComponent))
      (Rendering|Material|SetScalarParameterValue _returnvalue_5 "Luminosity" (Variables|Default|GetLuminosity) :!class /Script/Engine.MaterialInstanceDynamic)
      (Rendering|Material|SetScalarParameterValue _returnvalue_5 "Atmosphere_Intensity" (Variables|Default|GetAtmosphere_Intensity) :!class /Script/Engine.MaterialInstanceDynamic)
      (Rendering|Material|SetScalarParameterValue _returnvalue_5 "Cells_Intensity" (Variables|Default|GetCells_Intensity) :!class /Script/Engine.MaterialInstanceDynamic)
      (Rendering|Material|SetScalarParameterValue _returnvalue_5 "Flare_Intensity" (Variables|Default|GetFlare_Intensity) :!class /Script/Engine.MaterialInstanceDynamic)
      (Rendering|Material|SetVectorParameterValue _returnvalue_5 "Main_Color" (Variables|Default|GetMain_Color) :!class /Script/Engine.MaterialInstanceDynamic)
      (Rendering|Material|SetVectorParameterValue _returnvalue_5 "Atmosphere_Color" (Variables|Default|GetAtmosphere_Color) :!class /Script/Engine.MaterialInstanceDynamic)
      (Rendering|Material|SetVectorParameterValue _returnvalue_5 "Flare_Color" (Variables|Default|GetFlare_Color) :!class /Script/Engine.MaterialInstanceDynamic)
      (Rendering|Material|SetVectorParameterValue _returnvalue_5 "Cells_Color" (Variables|Default|GetCells_Color) :!class /Script/Engine.MaterialInstanceDynamic)
      (Rendering|Material|SetScalarParameterValue _returnvalue_5 "Cells_Count" (Variables|Default|GetCells_Count) :!class /Script/Engine.MaterialInstanceDynamic)
      (Rendering|Material|SetScalarParameterValue _returnvalue_5 "Fluid_Size" (Variables|Default|GetFluid_Size) :!class /Script/Engine.MaterialInstanceDynamic)
      (Rendering|Material|SetScalarParameterValue _returnvalue_5 "Atmosphere_Falloff" (Variables|Default|GetAtmosphere_Falloff) :!class /Script/Engine.MaterialInstanceDynamic)
      (Rendering|Material|SetTextureParameterValue _returnvalue_5 "Texture_Surface" (Variables|Default|GetTexture_Surface))
      (Rendering|Material|SetTextureParameterValue _returnvalue_5 "Texture_Randomizer_1" (Variables|Default|GetTexture_Randomizer_1))
      (Rendering|Material|SetTextureParameterValue _returnvalue_5 "Texture_Randomizer_2" (Variables|Default|GetTexture_Randomizer_2))
      (Rendering|Material|SetTextureParameterValue _returnvalue_5 "Texture_Flares" (Variables|Default|GetTexture_Flares))
      (Rendering|Material|SetTextureParameterValue _returnvalue_5 "Texture_ColdSpots" (Variables|Default|GetTexture_ColdSpots))
      (Rendering|Material|SetScalarParameterValue _returnvalue_5 "Surface_Warp_Intensity" (Variables|Default|GetSurface_Warp_Intensity) :!class /Script/Engine.MaterialInstanceDynamic))))

(fn ConstructionScript
  (bind _lens (Variables|Default|GetLens))
  (bind _main_particle (Variables|Default|GetMain_Particle))
  (bind _main_particle_2 (Variables|Default|GetMain_Particle))
  (bind _main_particle_3 (Variables|Default|GetMain_Particle))
  (bind _main_particle_4 (Variables|Default|GetMain_Particle))
  (bind _staticmesh (Variables|Default|GetStaticMesh))
  (bind _atmosphere_color (Variables|Default|GetAtmosphere_Color))
  (Utilities|FlowControl|Sequence
    (:then_0
      (bind _returnvalue (Rendering|Material|CreateDynamicMaterialInstance _main_particle 0 (Rendering|Material|GetMaterial _main_particle 0) "None" :!class /Script/Engine.PrimitiveComponent))
      (Variables|Default|SetDMI_Main_0 _returnvalue)
      (Rendering|Material|SetScalarParameterValue (Variables|Default|GetDMI_Main_0) "Opacity" (Variables|Default|GetRays_1) :!class /Script/Engine.MaterialInstanceDynamic)
      (Rendering|Material|SetVectorParameterValue (Variables|Default|GetDMI_Main_0) "Color" _atmosphere_color :!class /Script/Engine.MaterialInstanceDynamic))
    (:then_1
      (bind _returnvalue_2 (Rendering|Material|CreateDynamicMaterialInstance _main_particle_2 1 (Rendering|Material|GetMaterial _main_particle_2 1) "None" :!class /Script/Engine.PrimitiveComponent))
      (Variables|Default|SetDMI_Main_1 _returnvalue_2)
      (Rendering|Material|SetScalarParameterValue (Variables|Default|GetDMI_Main_1) "Opacity" (Variables|Default|GetRays_2) :!class /Script/Engine.MaterialInstanceDynamic)
      (Rendering|Material|SetVectorParameterValue (Variables|Default|GetDMI_Main_1) "Color" _atmosphere_color :!class /Script/Engine.MaterialInstanceDynamic))
    (:then_2
      (bind _returnvalue_3 (Rendering|Material|CreateDynamicMaterialInstance _main_particle_3 2 (Rendering|Material|GetMaterial _main_particle_3 2) "None" :!class /Script/Engine.PrimitiveComponent))
      (Variables|Default|SetDMI_Main_2 _returnvalue_3)
      (Rendering|Material|SetScalarParameterValue (Variables|Default|GetDMI_Main_2) "Opacity" (Variables|Default|GetRays_3) :!class /Script/Engine.MaterialInstanceDynamic)
      (Rendering|Material|SetVectorParameterValue (Variables|Default|GetDMI_Main_2) "Color" _atmosphere_color :!class /Script/Engine.MaterialInstanceDynamic))
    (:then_3
      (bind _returnvalue_4 (Rendering|Material|CreateDynamicMaterialInstance _main_particle_4 3 (Rendering|Material|GetMaterial _main_particle_4 3) "None" :!class /Script/Engine.PrimitiveComponent))
      (Variables|Default|SetDMI_Main_3 _returnvalue_4)
      (Rendering|Material|SetScalarParameterValue (Variables|Default|GetDMI_Main_3) "Opacity" (Variables|Default|GetRays_4) :!class /Script/Engine.MaterialInstanceDynamic)
      (Rendering|Material|SetVectorParameterValue (Variables|Default|GetDMI_Main_3) "Color" _atmosphere_color :!class /Script/Engine.MaterialInstanceDynamic))
    (:then_4
      (bind _returnvalue_5 (Rendering|Material|CreateDynamicMaterialInstance _staticmesh 0 (Rendering|Material|GetMaterial _staticmesh 0) "None" :!class /Script/Engine.PrimitiveComponent))
      (Rendering|Material|SetScalarParameterValue _returnvalue_5 "Luminosity" (Variables|Default|GetLuminosity) :!class /Script/Engine.MaterialInstanceDynamic)
      (Rendering|Material|SetScalarParameterValue _returnvalue_5 "Atmosphere_Intensity" (Variables|Default|GetAtmosphere_Intensity) :!class /Script/Engine.MaterialInstanceDynamic)
      (Rendering|Material|SetScalarParameterValue _returnvalue_5 "Cells_Intensity" (Variables|Default|GetCells_Intensity) :!class /Script/Engine.MaterialInstanceDynamic)
      (Rendering|Material|SetScalarParameterValue _returnvalue_5 "Flare_Intensity" (Variables|Default|GetFlare_Intensity) :!class /Script/Engine.MaterialInstanceDynamic)
      (Rendering|Material|SetVectorParameterValue _returnvalue_5 "Main_Color" (Variables|Default|GetMain_Color) :!class /Script/Engine.MaterialInstanceDynamic)
      (Rendering|Material|SetVectorParameterValue _returnvalue_5 "Atmosphere_Color" (Variables|Default|GetAtmosphere_Color) :!class /Script/Engine.MaterialInstanceDynamic)
      (Rendering|Material|SetVectorParameterValue _returnvalue_5 "Flare_Color" (Variables|Default|GetFlare_Color) :!class /Script/Engine.MaterialInstanceDynamic)
      (Rendering|Material|SetVectorParameterValue _returnvalue_5 "Cells_Color" (Variables|Default|GetCells_Color) :!class /Script/Engine.MaterialInstanceDynamic)
      (Rendering|Material|SetScalarParameterValue _returnvalue_5 "Cells_Count" (Variables|Default|GetCells_Count) :!class /Script/Engine.MaterialInstanceDynamic)
      (Rendering|Material|SetScalarParameterValue _returnvalue_5 "Fluid_Size" (Variables|Default|GetFluid_Size) :!class /Script/Engine.MaterialInstanceDynamic)
      (Rendering|Material|SetScalarParameterValue _returnvalue_5 "Atmosphere_Falloff" (Variables|Default|GetAtmosphere_Falloff) :!class /Script/Engine.MaterialInstanceDynamic)
      (Rendering|Material|SetTextureParameterValue _returnvalue_5 "Texture_Surface" (Variables|Default|GetTexture_Surface))
      (Rendering|Material|SetTextureParameterValue _returnvalue_5 "Texture_Randomizer_1" (Variables|Default|GetTexture_Randomizer_1))
      (Rendering|Material|SetTextureParameterValue _returnvalue_5 "Texture_Randomizer_2" (Variables|Default|GetTexture_Randomizer_2))
      (Rendering|Material|SetTextureParameterValue _returnvalue_5 "Texture_Flares" (Variables|Default|GetTexture_Flares))
      (Rendering|Material|SetTextureParameterValue _returnvalue_5 "Texture_ColdSpots" (Variables|Default|GetTexture_ColdSpots))
      (Rendering|Material|SetScalarParameterValue _returnvalue_5 "Surface_Warp_Intensity" (Variables|Default|GetSurface_Warp_Intensity) :!class /Script/Engine.MaterialInstanceDynamic))
    (:then_5
      (bind _returnvalue_6 (Rendering|Material|CreateDynamicMaterialInstance _lens 0 (Rendering|Material|GetMaterial _lens 0) "None" :!class /Script/Engine.PrimitiveComponent))
      (Rendering|Material|SetScalarParameterValue _returnvalue_6 "Lens_FadeDistance" (Variables|Default|GetLens_FadeDistance) :!class /Script/Engine.MaterialInstanceDynamic)
      (Rendering|Material|SetScalarParameterValue _returnvalue_6 "Lens_Intensity" (Variables|Default|GetLens_Intensity) :!class /Script/Engine.MaterialInstanceDynamic)
      (Rendering|Material|SetVectorParameterValue _returnvalue_6 "Color_1" (Variables|Default|GetMain_Color) :!class /Script/Engine.MaterialInstanceDynamic)
      (Rendering|Material|SetVectorParameterValue _returnvalue_6 "Color_2" (Variables|Default|GetOuterLens_Color) :!class /Script/Engine.MaterialInstanceDynamic))))